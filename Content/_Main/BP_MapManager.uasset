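; BP_MapManager is an actor that indexes the map's tiles and links them to their neighbours when play begins.
; It gathers every BP_TileBase actor into a list and records the one with the OriginForest gameplay tag as the origin tile.
; It then builds a coordinate-to-tile map and passes it to each tile's SetupNeigbours, so tiles resolve adjacency only after all coordinates are registered.
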(event `self.ReceiveBeginPlay`
  (bind _outactors (`GameplayStatics.GetAllActorsOfClass` "/Game/_Main/Level/LevelDesignElement/BP_TileBase.BP_TileBase_C"))
  (for _array_element _outactors
    (if (`BlueprintGameplayTagLibrary.HasTag` (`/Game/_Main/Level/LevelDesignElement/BP_TileBase.GameplayTags` _array_element) (struct :`TagName` "Tile.Type.OriginForest") true)
      (set `self.OriginTile` _array_element))
    (`KismetArrayLibrary.Array_Add` (`self.TileList`) _array_element))
  (for _array_element_2 (`self.TileList`)
    (`BlueprintMapLibrary.Map_Add` (`self.TileCoords`) (`/Game/_Main/Level/LevelDesignElement/BP_TileBase.Coords` _array_element_2) _array_element_2))
  (for _array_element_3 (`self.TileList`)
    (`/Game/_Main/Level/LevelDesignElement/BP_TileBase.SetupNeigbours` _array_element_3 (`self.TileCoords`))))

(fn `UserConstructionScript`)