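; Manager actor that applies card effects to map tiles in a forest-growing card game.
; PlayEffect routes an effect tag to tile stat boosts, sapling Growth, Replicate or Move, which tags valid forest targets for PlayerController targeting.
; CrossForestGrowth spreads forest to eligible orthogonal neighbours through the MapManager coordinate map.
; Tile updates swap Gameplay Tags and visual actors, with river variants and a reward for overgrowing human ruins.
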(event `self.ReceiveBeginPlay`
  (bind _asbp_player_controller (cast `/Game/_Main/BP_PlayerController` (`GameplayStatics.GetPlayerController` 0)))
  (set `self.Player Controller` _asbp_player_controller)
  (bind _asbp_game_instance (cast `/Game/_Main/BP_GameInstance` (`GameplayStatics.GetGameInstance`)))
  (set `self.Game Instance` _asbp_game_instance))

(fn `AbsorptionOnTarget`
  (params (Target :type "/Game/_Main/Level/LevelDesignElement/BP_TileBase Object Reference") (Power :type Integer))
  (bind (_tilestats_shield _tilestats_protection _tilestats_deeproots _tilestats_extraction _tilestats_frenzy _tilestats_absorption _tilestats_thorn) (break `/Game/_Main/Level/LevelDesignElement/S_TileStats` (`/Game/_Main/Level/LevelDesignElement/BP_TileBase.TileStats` Target)))
  (set `/Game/_Main/Level/LevelDesignElement/BP_TileBase.TileStats` (make `/Game/_Main/Level/LevelDesignElement/S_TileStats` _tilestats_shield _tilestats_protection _tilestats_deeproots _tilestats_extraction _tilestats_frenzy (+ Power _tilestats_absorption) _tilestats_thorn) Target)
  (`KismetSystemLibrary.PrintString` (`KismetStringLibrary.Concat_StrStr` "Absorption : " (`KismetStringLibrary.Conv_IntToString` _tilestats_absorption)) true true (struct :`G` 0.019376 :`B` 1.0 :`A` 1.0) 10.0))

(fn `CrossForestGrowth`
  (params (OriginTile :type "/Game/_Main/Level/LevelDesignElement/BP_TileBase Object Reference"))
  (bind (_coords_x _coords_y) (`KismetMathLibrary.BreakVector2D` (`/Game/_Main/Level/LevelDesignElement/BP_TileBase.Coords` OriginTile)))
  (bind _tilecoords (`/Game/_Main/BP_MapManager.TileCoords` (`/Game/_Main/BP_PlayerController.Map Manager` (`self.Player Controller`))))
  (`/Engine/EditorBlueprintResources/StandardMacros.IsValid` OriginTile
    (:`Is Valid`
      (for _array_element (`|MakeArray` (`BlueprintMapLibrary.Map_Find` _tilecoords (`KismetMathLibrary.MakeVector2D` _coords_x (+ _coords_y -100.0))) (`BlueprintMapLibrary.Map_Find` _tilecoords (`KismetMathLibrary.MakeVector2D` _coords_x (+ _coords_y 100.0))) (`BlueprintMapLibrary.Map_Find` _tilecoords (`KismetMathLibrary.MakeVector2D` (+ _coords_x 100.0) _coords_y)) (`BlueprintMapLibrary.Map_Find` _tilecoords (`KismetMathLibrary.MakeVector2D` (+ _coords_x -100.0) _coords_y)))
        (`/Engine/EditorBlueprintResources/StandardMacros.IsValid` _array_element
          (:`Is Valid`
            (bind _gameplaytags (`/Game/_Main/Level/LevelDesignElement/BP_TileBase.GameplayTags` _array_element))
            (if (not (or (`BlueprintGameplayTagLibrary.HasTag` _gameplaytags (struct :`TagName` "Tile.Type.Forest") true) (`BlueprintGameplayTagLibrary.HasTag` _gameplaytags (struct :`TagName` "Tile.Type.OriginForest") true) (`BlueprintGameplayTagLibrary.HasTag` _gameplaytags (struct :`TagName` "Sapling") true) (`BlueprintGameplayTagLibrary.HasTag` _gameplaytags (struct :`TagName` "Tile.Type.Mountain") true) (`BlueprintGameplayTagLibrary.HasTag` _gameplaytags (struct :`TagName` "Tile.Type.City") true) (`BlueprintGameplayTagLibrary.HasTag` _gameplaytags (struct :`TagName` "Tile.Type.Lumbercamp") true) (`BlueprintGameplayTagLibrary.HasTag` _gameplaytags (struct :`TagName` "Tile.Type.Village") true)))
              (bind _gameplaytags_2 (`/Game/_Main/Level/LevelDesignElement/BP_TileBase.GameplayTags` _array_element))
              (if (`BlueprintGameplayTagLibrary.HasTag` _gameplaytags_2 (struct :`TagName` "Tile.Type.River") true)
                (bind _returnvalue (`self.GetTransform` _array_element))
                (bind _waterforest (`self.SpawnWateredForest` _returnvalue))
                (`self.UpdateTileType` _waterforest _array_element)
                (`BlueprintGameplayTagLibrary.AddGameplayTag` (`/Game/_Main/Level/LevelDesignElement/BP_TileBase.GameplayTags` _array_element) (struct :`TagName` "Tile.Type.Forest"))
                (elif (`BlueprintGameplayTagLibrary.HasTag` _gameplaytags_2 (struct :`TagName` "Tile.Type.HumanRuins") true)
                  (`self.GrowOnRuins` _gameplaytags_2 _array_element)
                  (bind _forest (`self.SpawnForest` _returnvalue))
                  (`self.UpdateTileType` _forest _array_element)
                  (else
                    (`BlueprintGameplayTagLibrary.AddGameplayTag` _gameplaytags_2 (struct :`TagName` "Bush"))
                    (bind _forest_2 (`self.SpawnForest` _returnvalue))
                    (`self.UpdateTileType` _forest_2 _array_element))))
              (`/Game/_Main/Level/LevelDesignElement/BP_TileBase.Add HPs` _array_element 5)))))
      (`/Game/_Main/Level/LevelDesignElement/BP_TileBase.Add HPs` OriginTile 4))))

(fn `DeepRootOnTarget`
  (params (Target :type "/Game/_Main/Level/LevelDesignElement/BP_TileBase Object Reference") (Power :type Integer))
  (bind (_tilestats_shield _tilestats_protection _tilestats_deeproots _tilestats_extraction _tilestats_frenzy _tilestats_absorption _tilestats_thorn) (break `/Game/_Main/Level/LevelDesignElement/S_TileStats` (`/Game/_Main/Level/LevelDesignElement/BP_TileBase.TileStats` Target)))
  (set `/Game/_Main/Level/LevelDesignElement/BP_TileBase.TileStats` (make `/Game/_Main/Level/LevelDesignElement/S_TileStats` _tilestats_shield _tilestats_protection (+ Power _tilestats_deeproots) _tilestats_extraction _tilestats_frenzy _tilestats_absorption _tilestats_thorn) Target)
  (`KismetSystemLibrary.PrintString` (`KismetStringLibrary.Concat_StrStr` "DeepRoots : " (`KismetStringLibrary.Conv_IntToString` _tilestats_deeproots)) true true (struct :`G` 0.019376 :`B` 1.0 :`A` 1.0) 10.0))

(fn `ExtractionOnTarget`
  (params (Target :type "/Game/_Main/Level/LevelDesignElement/BP_TileBase Object Reference") (Power :type Integer))
  (bind (_tilestats_shield _tilestats_protection _tilestats_deeproots _tilestats_extraction _tilestats_frenzy _tilestats_absorption _tilestats_thorn) (break `/Game/_Main/Level/LevelDesignElement/S_TileStats` (`/Game/_Main/Level/LevelDesignElement/BP_TileBase.TileStats` Target)))
  (set `/Game/_Main/Level/LevelDesignElement/BP_TileBase.TileStats` (make `/Game/_Main/Level/LevelDesignElement/S_TileStats` _tilestats_shield _tilestats_protection _tilestats_deeproots (+ Power _tilestats_extraction) _tilestats_frenzy _tilestats_absorption _tilestats_thorn) Target)
  (`KismetSystemLibrary.PrintString` (`KismetStringLibrary.Concat_StrStr` "Extraction : " (`KismetStringLibrary.Conv_IntToString` _tilestats_extraction)) true true (struct :`G` 0.019376 :`B` 1.0 :`A` 1.0) 10.0))

(fn `FrenzyOnTarget`
  (params (Target :type "/Game/_Main/Level/LevelDesignElement/BP_TileBase Object Reference") (Power :type Integer))
  (bind (_tilestats_shield _tilestats_protection _tilestats_deeproots _tilestats_extraction _tilestats_frenzy _tilestats_absorption _tilestats_thorn) (break `/Game/_Main/Level/LevelDesignElement/S_TileStats` (`/Game/_Main/Level/LevelDesignElement/BP_TileBase.TileStats` Target)))
  (set `/Game/_Main/Level/LevelDesignElement/BP_TileBase.TileStats` (make `/Game/_Main/Level/LevelDesignElement/S_TileStats` _tilestats_shield _tilestats_protection _tilestats_deeproots _tilestats_extraction (+ Power _tilestats_frenzy) _tilestats_absorption _tilestats_thorn) Target)
  (`KismetSystemLibrary.PrintString` (`KismetStringLibrary.Concat_StrStr` "Frenzy : " (`KismetStringLibrary.Conv_IntToString` _tilestats_frenzy)) true true (struct :`G` 0.019376 :`B` 1.0 :`A` 1.0) 10.0))

(fn `GrowOnRuins`
  (params (TagContainer :type "GameplayTagContainer Structure (by ref)") (TileToUpdate :type "/Game/_Main/Level/LevelDesignElement/BP_TileBase Object Reference"))
  (set `/Game/_Main/Level/LevelDesignElement/BP_TileBase.TileTypeVisual` null TileToUpdate)
  (`BlueprintGameplayTagLibrary.AddGameplayTag` TagContainer (struct :`TagName` "Bush"))
  (`BlueprintGameplayTagLibrary.RemoveGameplayTag` TagContainer (struct :`TagName` "Tile.Type.HumanRuins"))
  (`/Game/_Main/BP_PlayerController.Get a Reward` (`self.Player Controller`)))

(fn `Growth`
  (params (OriginTile :type "/Game/_Main/Level/LevelDesignElement/BP_TileBase Object Reference") (SaplingToGrowth :type Name))
  (bind _saplingtogrowthdata (`/Game/_Main/BP_GameInstance.GetSapling(RowName)` (`self.Game Instance`) SaplingToGrowth))
  (bind _returnvalue (`|SpawnActorFromClass` "/Game/_Main/Actors/Saplings/BP_Sapling.BP_Sapling_C" (`KismetMathLibrary.MakeTransform` (`self.K2_GetActorLocation` OriginTile)) "Undefined" "MultiplyWithRoot" null OriginTile _saplingtogrowthdata null null null null))
  (`self.UpdateTileSapling` _returnvalue OriginTile))

(fn `Move`
  (params (Target :type "/Game/_Main/Level/LevelDesignElement/BP_TileBase Object Reference") (Power :type Integer))
  (bind _player_controller (`self.Player Controller`))
  (set `/Game/_Main/BP_PlayerController.CurrentTileSelected` Target (`self.Player Controller`))
  (set `/Game/_Main/BP_PlayerController.PlayingCardEffect` Power _player_controller)
  (set `/Game/_Main/BP_PlayerController.MooveEffect` "NewEnumerator13" _player_controller)
  (bind _tileinrange (`/Game/_Main/BP_PlayerController.FindTargetInRadiusOfATile` _player_controller (`local.Target`) (* Power 100)))
  (for _array_element _tileinrange
    (bind _gameplaytags (`/Game/_Main/Level/LevelDesignElement/BP_TileBase.GameplayTags` _array_element))
    (if (not (or (`BlueprintGameplayTagLibrary.HasTag` _gameplaytags (struct :`TagName` "Sapling.Attack") true) (`BlueprintGameplayTagLibrary.HasTag` _gameplaytags (struct :`TagName` "Sapling.Mana") true)))
      (if (`BlueprintGameplayTagLibrary.HasTag` _gameplaytags (struct :`TagName` "Tile.Type.Forest") true)
        (`BlueprintGameplayTagLibrary.AddGameplayTag` (`/Game/_Main/Level/LevelDesignElement/BP_TileBase.GameplayTags` _array_element) (struct :`TagName` "Tile.Target.IsValid")))))
  (`/Game/_Main/BP_PlayerController.SpawnTargettingActor` (`self.Player Controller`)))

(fn `PlayEffect`
  (params (Target :type "/Game/_Main/Level/LevelDesignElement/BP_TileBase Object Reference") (TagToUse :type "/Game/_Main/TCG/Cards/Data/E_Tags Enum" :default "NewEnumerator1") (Power :type Integer) (SaplingToGrowth :type Name))
  (switch `/Game/_Main/TCG/Cards/Data/E_Tags` TagToUse
    (:`NewEnumerator0`
      (`self.ShieldOnTarget` (`local.Target`) (`local.Power`)))
    (:`NewEnumerator2`
      (`self.ProtectionOnTarget` (`local.Target`) (`local.Power`)))
    (:`NewEnumerator3`
      (`self.Move` (`local.Target`) (`local.Power`)))
    (:`NewEnumerator6`
      (`self.Replicate` (`local.Power`)))
    (:`NewEnumerator7`
      (`self.DeepRootOnTarget` (`local.Target`) (`local.Power`)))
    (:`NewEnumerator8`
      (`self.ExtractionOnTarget` (`local.Target`) (`local.Power`)))
    (:`NewEnumerator10`
      (`self.FrenzyOnTarget` (`local.Target`) (`local.Power`)))
    (:`NewEnumerator20`
      (`self.ThornOnTarget` (`local.Target`) (`local.Power`)))
    (:`NewEnumerator21`
      (`self.Growth` (`local.Target`) (`local.SaplingToGrowth`)))))

(fn `ProtectionOnTarget`
  (params (Target :type "/Game/_Main/Level/LevelDesignElement/BP_TileBase Object Reference") (Power :type Integer))
  (bind (_tilestats_shield _tilestats_protection _tilestats_deeproots _tilestats_extraction _tilestats_frenzy _tilestats_absorption _tilestats_thorn) (break `/Game/_Main/Level/LevelDesignElement/S_TileStats` (`/Game/_Main/Level/LevelDesignElement/BP_TileBase.TileStats` Target)))
  (set `/Game/_Main/Level/LevelDesignElement/BP_TileBase.TileStats` (make `/Game/_Main/Level/LevelDesignElement/S_TileStats` _tilestats_shield (+ Power _tilestats_protection) _tilestats_deeproots _tilestats_extraction _tilestats_frenzy _tilestats_absorption _tilestats_thorn) Target)
  (`KismetSystemLibrary.PrintString` (`KismetStringLibrary.Concat_StrStr` "Protection : " (`KismetStringLibrary.Conv_IntToString` _tilestats_protection)) true true (struct :`G` 0.019376 :`B` 1.0 :`A` 1.0) 10.0))

(fn `RemovePreviousTileType`
  (params (TileToUpdate :type "/Game/_Main/Level/LevelDesignElement/BP_TileBase Object Reference"))
  (bind _gameplaytags (`/Game/_Main/Level/LevelDesignElement/BP_TileBase.GameplayTags` TileToUpdate))
  (for _array_element (`BlueprintGameplayTagLibrary.BreakGameplayTagContainer` _gameplaytags)
    (if (and (`BlueprintGameplayTagLibrary.MatchesTag` _array_element (struct :`TagName` "Tile.Type")) (not (`BlueprintGameplayTagLibrary.MatchesTag` _array_element (struct :`TagName` "Tile.Type.HumanRuins") true)))
      (`BlueprintGameplayTagLibrary.RemoveGameplayTag` _gameplaytags _array_element)))
  (return))

(fn `Replicate`
  (params (Power :type Integer))
  (set `/Game/_Main/BP_PlayerState.Replicate?` true (`/Game/_Main/BP_PlayerController.Player State` (`self.Player Controller`))))

(fn `ShieldOnTarget`
  (params (Target :type "/Game/_Main/Level/LevelDesignElement/BP_TileBase Object Reference") (Power :type Integer))
  (bind (_tilestats_shield _tilestats_protection _tilestats_deeproots _tilestats_extraction _tilestats_frenzy _tilestats_absorption _tilestats_thorn) (break `/Game/_Main/Level/LevelDesignElement/S_TileStats` (`/Game/_Main/Level/LevelDesignElement/BP_TileBase.TileStats` Target)))
  (set `/Game/_Main/Level/LevelDesignElement/BP_TileBase.TileStats` (make `/Game/_Main/Level/LevelDesignElement/S_TileStats` (+ Power _tilestats_shield) _tilestats_protection _tilestats_deeproots _tilestats_extraction _tilestats_frenzy _tilestats_absorption _tilestats_thorn) Target)
  (`KismetSystemLibrary.PrintString` (`KismetStringLibrary.Concat_StrStr` "Shield : " (`KismetStringLibrary.Conv_IntToString` _tilestats_shield)) true true (struct :`G` 0.019376 :`B` 1.0 :`A` 1.0) 10.0))

(fn `SpawnForest`
  (params (TileLocation :type "Transform Structure"))
  (returns (Forest :type "/Game/_Main/Actors/Forest/ForestPart/BP_Foresst Object Reference"))
  (bind _returnvalue (`|SpawnActorFromClass` "/Game/_Main/Actors/Forest/ForestPart/BP_Foresst.BP_Foresst_C" TileLocation "Undefined" "MultiplyWithRoot" null null null null null))
  (return _returnvalue))

(fn `SpawnVillage`
  (params (TileLocation :type "Transform Structure"))
  (returns (Village :type "/Game/_Main/Actors/Enemy/BP_BaseEnemyBuild Object Reference"))
  (bind _returnvalue (`|SpawnActorFromClass` "/Game/_Main/Actors/Enemy/BP_BaseEnemyBuild.BP_BaseEnemyBuild_C" TileLocation "Undefined" "MultiplyWithRoot" null null null null null null))
  (return _returnvalue))

(fn `SpawnWateredForest`
  (params (TileLocation :type "Transform Structure"))
  (returns (WaterForest :type "/Game/_Main/Actors/Forest/ForestPart/BP_WaterForest Object Reference"))
  (bind _returnvalue (`|SpawnActorFromClass` "/Game/_Main/Actors/Forest/ForestPart/BP_WaterForest.BP_WaterForest_C" TileLocation "Undefined" "MultiplyWithRoot" null null null null null))
  (return _returnvalue))

(fn `ThornOnTarget`
  (params (Target :type "/Game/_Main/Level/LevelDesignElement/BP_TileBase Object Reference") (Power :type Integer))
  (bind (_tilestats_shield _tilestats_protection _tilestats_deeproots _tilestats_extraction _tilestats_frenzy _tilestats_absorption _tilestats_thorn) (break `/Game/_Main/Level/LevelDesignElement/S_TileStats` (`/Game/_Main/Level/LevelDesignElement/BP_TileBase.TileStats` Target)))
  (set `/Game/_Main/Level/LevelDesignElement/BP_TileBase.TileStats` (make `/Game/_Main/Level/LevelDesignElement/S_TileStats` _tilestats_shield _tilestats_protection _tilestats_deeproots _tilestats_extraction _tilestats_frenzy _tilestats_absorption (+ Power _tilestats_thorn)) Target)
  (`KismetSystemLibrary.PrintString` (`KismetStringLibrary.Concat_StrStr` "Thorn : " (`KismetStringLibrary.Conv_IntToString` _tilestats_thorn)) true true (struct :`G` 0.019376 :`B` 1.0 :`A` 1.0) 10.0))

(fn `UpdateTileBush`
  (params (TileActorToAdd :type "/Game/_Main/Actors/Saplings/BP_Bush Object Reference") (`Tile To Update` :type "/Game/_Main/Level/LevelDesignElement/BP_TileBase Object Reference"))
  (locals (`TempTile&LinkedActor` :type "Map of /Game/_Main/Level/LevelDesignElement/BP_TileBase Object Reference to /Game/_Main/Actors/Struct/S_TileActor Structure"))
  (set `/Game/_Main/Level/LevelDesignElement/BP_TileBase.Sapling` TileActorToAdd `Tile To Update`)
  (`BlueprintGameplayTagLibrary.AddGameplayTag` (`/Game/_Main/Level/LevelDesignElement/BP_TileBase.GameplayTags` (`local.Tile To Update`)) (struct :`TagName` "Bush"))
  (if (`BlueprintGameplayTagLibrary.HasTag` (`/Game/_Main/Level/LevelDesignElement/BP_TileBase.GameplayTags` `Tile To Update`) (struct :`TagName` "Tile.Type.River") true)
    (bind _returnvalue (`|SpawnActorFromClass` "/Game/_Main/Actors/Forest/ForestPart/BP_WaterForest.BP_WaterForest_C" (`self.GetTransform` (`local.Tile To Update`)) "Undefined" "MultiplyWithRoot" null null null null null))
    (set `/Game/_Main/Level/LevelDesignElement/BP_TileBase.TileTypeVisual` _returnvalue (`local.Tile To Update`))
    (else
      (bind _returnvalue_2 (`|SpawnActorFromClass` "/Game/_Main/Actors/Forest/ForestPart/BP_VisualBush.BP_VisualBush_C" (`self.GetTransform` (`local.Tile To Update`)) "Undefined" "MultiplyWithRoot" null null null null null))
      (set `/Game/_Main/Level/LevelDesignElement/BP_TileBase.TileTypeVisual` _returnvalue_2 (`local.Tile To Update`))))
  (`/Game/_Main/Level/LevelDesignElement/BP_TileBase.UpdateMaterial` (`local.Tile To Update`)))

(fn `UpdateTileSapling`
  (params (TileActorToAdd :type "/Game/_Main/Actors/Saplings/BP_Sapling Object Reference") (`Tile To Update` :type "/Game/_Main/Level/LevelDesignElement/BP_TileBase Object Reference"))
  (locals (`TempTile&LinkedActor` :type "Map of /Game/_Main/Level/LevelDesignElement/BP_TileBase Object Reference to /Game/_Main/Actors/Struct/S_TileActor Structure") (TileVisual :type "/Game/_Main/Actors/Forest/ForestPart/BP_VisualBush Object Reference") (TileVisuaBase :type "/Game/_Main/Actors/Forest/ForestPart/BP_Foresst Object Reference"))
  (bind _tile_to_update (`local.Tile To Update`))
  (bind _gameplaytags (`/Game/_Main/Level/LevelDesignElement/BP_TileBase.GameplayTags` (`local.Tile To Update`)))
  (bind _gameplaytags_2 (`/Game/_Main/Level/LevelDesignElement/BP_TileBase.GameplayTags` (`local.Tile To Update`)))
  (set `/Game/_Main/Level/LevelDesignElement/BP_TileBase.Sapling` TileActorToAdd `Tile To Update`)
  (`BlueprintGameplayTagLibrary.AddGameplayTag` (`/Game/_Main/Level/LevelDesignElement/BP_TileBase.GameplayTags` `Tile To Update`) (struct :`TagName` "Sapling"))
  (if (`BlueprintGameplayTagLibrary.HasTag` _gameplaytags_2 (struct :`TagName` "Bush") true)
    (`BlueprintGameplayTagLibrary.RemoveGameplayTag` _gameplaytags_2 (struct :`TagName` "Bush"))
    (elif (not (`BlueprintGameplayTagLibrary.HasTag` _gameplaytags_2 (struct :`TagName` "Tile.Type.River") true))
      (`self.RemovePreviousTileType` (`local.Tile To Update`))))
  (`BlueprintGameplayTagLibrary.AddGameplayTag` _gameplaytags_2 (struct :`TagName` "Tile.Type.Forest"))
  (if (`BlueprintGameplayTagLibrary.HasTag` _gameplaytags (struct :`TagName` "Tile.Type.HumanRuins"))
    (`self.GrowOnRuins` _gameplaytags))
  (if (not (>= (`.ForestMaxHP_22_A74711E54DD60A25A9CC27B1D81B1D2D` (break `/Game/_Main/Level/LevelDesignElement/S_TileStats` (`/Game/_Main/Level/LevelDesignElement/BP_TileBase.TileStats` (`local.Tile To Update`)))) 5))
    (`/Game/_Main/Level/LevelDesignElement/BP_TileBase.Add HPs` _tile_to_update 1))
  (`/Game/_Main/Level/LevelDesignElement/BP_TileBase.UpdateMaterial` _tile_to_update))

(fn `UpdateTileType`
  (params (TileActorToAdd :type "/Game/_Main/Actors/BP_TileActor Object Reference") (`Tile To Update` :type "/Game/_Main/Level/LevelDesignElement/BP_TileBase Object Reference"))
  (locals (`TempTile&LinkedActor` :type "Map of /Game/_Main/Level/LevelDesignElement/BP_TileBase Object Reference to /Game/_Main/Actors/Struct/S_TileActor Structure"))
  (bind _tile_to_update (`local.Tile To Update`))
  (bind _tiletypevisual (`/Game/_Main/Level/LevelDesignElement/BP_TileBase.TileTypeVisual` `Tile To Update`))
  (bind _tile_to_update_2 (`local.Tile To Update`))
  (bind _gameplaytags (`/Game/_Main/Level/LevelDesignElement/BP_TileBase.GameplayTags` _tile_to_update))
  ; Sert à supprimer l'ancien visuel
  (`/Engine/EditorBlueprintResources/StandardMacros.IsValid` _tiletypevisual
    (:`Is Valid`
      (`self.K2_DestroyActor` _tiletypevisual))
    (:`Is Not Valid`
      _))
  (bind _output_get (set `/Game/_Main/Level/LevelDesignElement/BP_TileBase.TileTypeVisual` TileActorToAdd _tile_to_update_2))
  (`self.RemovePreviousTileType` _tile_to_update_2)
  (`BlueprintGameplayTagLibrary.AddGameplayTag` (`/Game/_Main/Level/LevelDesignElement/BP_TileBase.GameplayTags` (`local.Tile To Update`)) (`/Game/_Main/Actors/BP_TileActor.TileVisual_GPTag` _output_get))
  (`/Game/_Main/Level/LevelDesignElement/BP_TileBase.UpdateMaterial` _tile_to_update)
  (if (and (`BlueprintGameplayTagLibrary.HasTag` _gameplaytags (struct :`TagName` "Tile.Type.Forest") true) (`BlueprintGameplayTagLibrary.HasTag` _gameplaytags (struct :`TagName` "Tile.State.AdjacentToForest") true))
    (`BlueprintGameplayTagLibrary.RemoveGameplayTag` _gameplaytags (struct :`TagName` "Tile.State.AdjacentToForest"))))

(fn `UserConstructionScript`)