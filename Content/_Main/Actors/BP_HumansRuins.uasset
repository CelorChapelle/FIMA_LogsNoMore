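; BP_HumansRuins is the actor that turns a map tile into human ruins.
; On BeginPlay it registers itself as the linked tile decor's Ruins and TileTypeVisual, adds the HumanRuins tag and strips lumber camp, village and city tags, both tile-type and enemy-building.
; It then has the tile decor update its material before calling the parent BeginPlay.
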(event `self.ReceiveBeginPlay`
  (bind _linkedtiledecor (`self.LinkedTileDecor`))
  (bind _gameplaytags (`/Game/_Main/Level/LevelDesignElement/BP_TileBase.GameplayTags` _linkedtiledecor))
  (set `/Game/_Main/Level/LevelDesignElement/BP_TileBase.Ruins` self _linkedtiledecor)
  (set `/Game/_Main/Level/LevelDesignElement/BP_TileBase.TileTypeVisual` self _linkedtiledecor)
  (`BlueprintGameplayTagLibrary.AddGameplayTag` _gameplaytags (struct :`TagName` "Tile.Type.HumanRuins"))
  (`BlueprintGameplayTagLibrary.RemoveGameplayTag` _gameplaytags (struct :`TagName` "Ennemi.Building.LumberCamp"))
  (`BlueprintGameplayTagLibrary.RemoveGameplayTag` _gameplaytags (struct :`TagName` "Tile.Type.Lumbercamp"))
  (`BlueprintGameplayTagLibrary.RemoveGameplayTag` _gameplaytags (struct :`TagName` "Ennemi.Building.Village"))
  (`BlueprintGameplayTagLibrary.RemoveGameplayTag` _gameplaytags (struct :`TagName` "Tile.Type.Village"))
  (`BlueprintGameplayTagLibrary.RemoveGameplayTag` _gameplaytags (struct :`TagName` "Ennemi.Building.City"))
  (`BlueprintGameplayTagLibrary.RemoveGameplayTag` _gameplaytags (struct :`TagName` "Tile.Type.City"))
  (`/Game/_Main/Level/LevelDesignElement/BP_TileBase.UpdateTileMaterial` _linkedtiledecor)
  (`parent.ReceiveBeginPlay`))

(fn `UserConstructionScript`
  (`parent.UserConstructionScript`))