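; BP_Village is an enemy village on the tile map that spawns lumberjack minions during the enemy turn.
; ExecuteEnemiTurn scans a square of tiles within AlertRadius, through the MapManager's coordinate map, for Forest or AdjacentToForest gameplay tags.
; If forest is found, the unit count is below MaxUnits and its tile has no minion, it spawns a BP_LumberJackBase there and tags the tile.
; GetEnemiTurnPriority exposes its turn priority.
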(event `self.ReceiveBeginPlay`)

(event `/Game/_Main/BPI_EnemiTurn.Execute Enemi Turn`
  (`self.ForestDetection`))

(fn `ForestDetection`
  (bind _parenttile (`self.ParentTile`))
  (bind _alertradius (`self.AlertRadius`))
  (bind (_coords_x _coords_y) (`KismetMathLibrary.BreakVector2D` (`/Game/_Main/Level/LevelDesignElement/BP_TileBase.Coords` _parenttile)))
  (for _index (range (* _alertradius -1) (+ _alertradius 1))
    (for _index_2 (range (* _alertradius -1) (+ _alertradius 1))
      (bind _value (`BlueprintMapLibrary.Map_Find` (`/Game/_Main/BP_MapManager.TileCoords` (`/Game/_Main/BP_PlayerController.Map Manager` (`/Game/_Main/Level/LevelDesignElement/BP_TileBase.Player Controller` _parenttile))) (`KismetMathLibrary.MakeVector2D` (+ _coords_x (* _index 100)) (+ _coords_y (* _index_2 100)))))
      (`/Engine/EditorBlueprintResources/StandardMacros.IsValid` _value
        (:`Is Valid`
          (bind _gameplaytags (`/Game/_Main/Level/LevelDesignElement/BP_TileBase.GameplayTags` _value))
          (if (or (`BlueprintGameplayTagLibrary.HasTag` _gameplaytags (struct :`TagName` "Tile.State.AdjacentToForest") true) (`BlueprintGameplayTagLibrary.HasTag` _gameplaytags (struct :`TagName` "Tile.Type.Forest") true))
            (set `self.CanSpawn` true))))))
  (if (and (`self.CanSpawn`) (< (`self.ActualsUnits`) (`self.MaxUnits`)) (not (`KismetSystemLibrary.IsValid` (`/Game/_Main/Level/LevelDesignElement/BP_TileBase.EnemyMinion` (`self.ParentTile`)))))
    (`self.SpawnLumberJack`)
    (set `self.CanSpawn` false)))

(fn `GetEnemiTurnPriority`
  (returns (Priority :type Integer))
  (return (`self.TurnPriority`)))

(fn `SpawnLumberJack`
  (bind _parenttile (`self.ParentTile`))
  (bind _parenttile_2 (`self.ParentTile`))
  (bind _returnvalue (`|SpawnActorFromClass` "/Game/_Main/Actors/Enemi/BP_LumberJackBase.BP_LumberJackBase_C" (`self.GetTransform` _parenttile) "Undefined" "MultiplyWithRoot" null _parenttile null))
  (set `self.ActualsUnits` (+ (`self.ActualsUnits`) 1))
  (set `/Game/_Main/Level/LevelDesignElement/BP_TileBase.EnemyMinion` _returnvalue _parenttile_2)
  (`BlueprintGameplayTagLibrary.AddGameplayTag` (`/Game/_Main/Level/LevelDesignElement/BP_TileBase.GameplayTags` _parenttile_2) (struct :`TagName` "Ennemi.Minion.LumberJack")))

(fn `UserConstructionScript`)