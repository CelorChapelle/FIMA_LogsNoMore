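; BP_Boomcap is a mine-like sapling that occupies a tile's Boomcap slot and swaps that tile's Trap tag for Boomcap.
; On its turn, if an enemy minion is on its tile or a neighbor, it damages tagged minions on neighboring tiles, restores the tags and destroys itself.
; A kill has roughly even odds of spawning another Boomcap on the victim's free slot.
; FindTarget and Fire are defined but not called here.
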(event `self.ReceiveBeginPlay`
  (bind _linkedtile_0 (`self.LinkedTile_0`))
  (bind (_sapling _turntogrowth _initiative _overviewtext _tags _canattack_ _damage) (break `/Game/_Main/TCG/Cards/Data/S_Saplings` (`self.SaplingInfos`)))
  (bind _gameplaytags (`/Game/_Main/Level/LevelDesignElement/BP_TileBase.GameplayTags` _linkedtile_0))
  (`parent.ReceiveBeginPlay`)
  (set `self.Priority` _initiative)
  (set `self.Damage` _damage)
  (set `/Game/_Main/Level/LevelDesignElement/BP_TileBase.Boomcapslot` self _linkedtile_0)
  (`BlueprintGameplayTagLibrary.AddGameplayTag` _gameplaytags (struct :`TagName` "Sapling.Boomcap"))
  (`BlueprintGameplayTagLibrary.RemoveGameplayTag` _gameplaytags (struct :`TagName` "Sapling.Trap")))

(event `self.Execute Player Turn`
  (bind _linkedtile_0 (`self.LinkedTile_0`))
  (bind _gameplaytags (`/Game/_Main/Level/LevelDesignElement/BP_TileBase.GameplayTags` _linkedtile_0))
  (bind _canexplode__ (`self.CanExplode ?`))
  (if _canexplode__
    (`self.Attack` null)
    (set `/Game/_Main/Level/LevelDesignElement/BP_TileBase.Boomcapslot` null _linkedtile_0)
    (`BlueprintGameplayTagLibrary.RemoveGameplayTag` _gameplaytags (struct :`TagName` "Sapling.Boomcap"))
    (`BlueprintGameplayTagLibrary.AddGameplayTag` _gameplaytags (struct :`TagName` "Sapling.Trap"))
    (`self.K2_DestroyActor`)))

(event `/Game/_Main/BPI_OnKill.OnKill`
  (params (KilledActor :type "/Game/_Main/Actors/Enemy/BP_LumberJackBase Object Reference"))
  (bind _currenttile (`/Game/_Main/Actors/Enemy/BP_LumberJackBase.CurrentTile` KilledActor))
  (`/Engine/EditorBlueprintResources/StandardMacros.IsValid` (`/Game/_Main/Level/LevelDesignElement/BP_TileBase.Boomcapslot` _currenttile)
    (:`Is Not Valid`
      (if (>= (`KismetMathLibrary.RandomIntegerInRange` 0 100) 50)
        (bind _returnvalue (`|SpawnActorFromClass` "BP_Boomcap_C" (`KismetMathLibrary.Conv_VectorToTransform` (`self.K2_GetActorLocation` _currenttile)) "Undefined" "MultiplyWithRoot" null _currenttile (`self.SaplingInfos`) null null null null))
        (set `/Game/_Main/Level/LevelDesignElement/BP_TileBase.Boomcapslot` _returnvalue (`/Game/_Main/Actors/Enemy/BP_LumberJackBase.CurrentTile` KilledActor))))))

(fn `Attack`
  (params (Target :type "/Game/_Main/Level/LevelDesignElement/BP_TileBase Object Reference"))
  (for _array_element (`/Game/_Main/Level/LevelDesignElement/BP_TileBase.Voisins` (`self.LinkedTile_0`))
    (`/Engine/EditorBlueprintResources/StandardMacros.IsValid` _array_element
      (:`Is Valid`
        (if (`BlueprintGameplayTagLibrary.HasTag` (`/Game/_Main/Level/LevelDesignElement/BP_TileBase.GameplayTags` _array_element) (struct :`TagName` "Ennemi.Minion"))
          (bind _enemyminion (`/Game/_Main/Level/LevelDesignElement/BP_TileBase.EnemyMinion` _array_element))
          (`/Engine/EditorBlueprintResources/StandardMacros.IsValid` _enemyminion
            (:`Is Valid`
              (`GameplayStatics.ApplyDamage` _enemyminion (`KismetMathLibrary.Conv_IntToDouble` (`self.Damage`)) null self))))))))

(fn `CanExplode ?`
  (returns (`CanExplode ?` :type Boolean))
  (locals (CanExplode :type Boolean))
  (bind _linkedtile_0 (`self.LinkedTile_0`))
  (set `local.CanExplode` false)
  (`/Engine/EditorBlueprintResources/StandardMacros.IsValid` (`/Game/_Main/Level/LevelDesignElement/BP_TileBase.EnemyMinion` _linkedtile_0)
    (:`Is Valid`
      (set `local.CanExplode` true))
    (:`Is Not Valid`
      (for _array_element (`/Game/_Main/Level/LevelDesignElement/BP_TileBase.Voisins` _linkedtile_0)
        (`/Engine/EditorBlueprintResources/StandardMacros.IsValid` _array_element
          (:`Is Valid`
            (`/Engine/EditorBlueprintResources/StandardMacros.IsValid` (`/Game/_Main/Level/LevelDesignElement/BP_TileBase.EnemyMinion` _array_element)
              (:`Is Valid`
                (set `local.CanExplode` true)
                (break))))))))
  (return (`local.CanExplode`)))

(fn `FindTarget`
  (returns (Target :type "/Game/_Main/Level/LevelDesignElement/BP_TileBase Object Reference"))
  (locals (PotentialTargets :type "Array of /Game/_Main/Level/LevelDesignElement/BP_TileBase Object Reference") (BestTarget :type "/Game/_Main/Level/LevelDesignElement/BP_TileBase Object Reference") (BestDistance :type "Float (double-precision)") (BestTargetPriority :type Integer) (BestTagPriority :type Integer) (BestGameplayTag :type "GameplayTag Structure"))
  (bind _besttagpriority (`local.BestTagPriority`))
  (bind _potentialtargets (`local.PotentialTargets`))
  (bind _returnvalue (`self.K2_GetActorLocation` (`self.LinkedTile_0`)))
  (`|ExecutionSequence`
    (:`then_0`
      (bind _outhits (`KismetSystemLibrary.SphereTraceMultiForObjects` :`Start` _returnvalue :`End` _returnvalue :`Radius` (`KismetMathLibrary.Conv_IntToDouble` (`.RangeMax_40_3ACA23034E250E9CBD201D9D1F74DF94` (break `/Game/_Main/TCG/Cards/Data/S_Saplings` (`self.SaplingInfos`)))) :`ObjectTypes` (`|MakeArray` "ObjectTypeQuery7" :!type "EObjectTypeQuery Enum") :`DrawDebugType` "ForDuration"))
      (for _array_element _outhits
        (bind _asbp_tile_base (cast `/Game/_Main/Level/LevelDesignElement/BP_TileBase` (`.HitActor` (`GameplayStatics.BreakHitResult` _array_element))))
        (if (`BlueprintGameplayTagLibrary.HasTag` (`/Game/_Main/Level/LevelDesignElement/BP_TileBase.GameplayTags` _asbp_tile_base) (struct :`TagName` "Ennemi"))
          (`KismetArrayLibrary.Array_Add` (`local.PotentialTargets`) _asbp_tile_base))))
    (:`then_1`
      (set `local.BestGameplayTag` (struct))
      (set `local.BestTagPriority` 999)
      (set `local.BestTargetPriority` 999)
      (set `local.BestDistance` 9999999999.0)
      (set `local.BestTarget` null)
      (if (`KismetArrayLibrary.Array_IsNotEmpty` _potentialtargets)
        (for _array_element_2 _potentialtargets
          (bind _returnvalue_2 (`KismetMathLibrary.Vector_DistanceSquared` (`self.K2_GetActorLocation` _array_element_2) (`self.K2_GetActorLocation` (`self.LinkedTile_0`))))
          (if (< _returnvalue_2 (`local.BestDistance`))
            (for _array_element_3 (`BlueprintGameplayTagLibrary.BreakGameplayTagContainer` (`/Game/_Main/Level/LevelDesignElement/BP_TileBase.GameplayTags` _array_element_2))
              (bind (_value _returnvalue_3) (`BlueprintMapLibrary.Map_Find` (`self.TargetPriority`) _array_element_3))
              (if (and _returnvalue_3 (< _value (`local.BestTagPriority`)))
                (set `local.BestTagPriority` _value)
                (set `local.BestGameplayTag` _array_element_3)))
            (if (< _besttagpriority (`local.BestTargetPriority`))
              (set `local.BestTargetPriority` _besttagpriority)
              (set `local.BestDistance` _returnvalue_2)
              (set `local.BestTarget` _array_element_2))))
        (return (`local.BestTarget`))))))

(fn `Fire`
  (params (Target :type "/Game/_Main/Level/LevelDesignElement/BP_TileBase Object Reference"))
  (`/Engine/EditorBlueprintResources/StandardMacros.IsValid` Target
    (:`Is Valid`
      (`|SpawnActorFromClass` "/Game/_Main/Actors/Saplings/Projectile/BP_BaseProjectile.BP_BaseProjectile_C" (`self.GetTransform`) "Undefined" "MultiplyWithRoot" null (`self.K2_GetActorLocation`) (`self.K2_GetActorLocation` Target) (`self.TurnTime`) null))))

(fn `UserConstructionScript`)