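; BP_Fountain is a sapling building that raises the player's card draw per turn while it stands.
; On BeginPlay it takes its priority from its initiative stat, registers on its linked tile, refreshes the tile's sapling type and adds HP to it.
; It then increments the draw count on the tile's PlayerController, and its DestroySapling override reverses that bonus before running the parent teardown.
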(event `self.ReceiveBeginPlay`
  (bind _linkedtile_0 (`self.LinkedTile_0`))
  (`parent.ReceiveBeginPlay`)
  (set `self.Priority` (`.Initiative_67_8E3A803442548E530550E9B0BE977E07` (break `/Game/_Main/TCG/Cards/Data/S_Saplings` (`self.SaplingInfos`))))
  (set `/Game/_Main/Level/LevelDesignElement/BP_TileBase.SaplingBuilding` self _linkedtile_0)
  (`/Game/_Main/Level/LevelDesignElement/BP_TileBase.Update SaplingType` _linkedtile_0)
  (`/Game/_Main/Level/LevelDesignElement/BP_TileBase.Add HPs` _linkedtile_0 3)
  (`/Game/_Main/BP_PlayerController.UpdateDrawCardPerTurn` (`/Game/_Main/Level/LevelDesignElement/BP_TileBase.Player Controller` (`self.LinkedTile_0`)) 1))

(fn `DestroySapling`
  (`/Game/_Main/BP_PlayerController.UpdateDrawCardPerTurn` (`/Game/_Main/Level/LevelDesignElement/BP_TileBase.Player Controller` (`self.LinkedTile_0`)) -1)
  (`parent.DestroySapling`))

(fn `UserConstructionScript`
  (`parent.UserConstructionScript`))