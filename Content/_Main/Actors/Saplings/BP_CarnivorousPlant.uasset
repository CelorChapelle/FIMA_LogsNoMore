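; Carnivorous plant sapling that attacks enemy minions and buildings within range on the player's turn.
; On BeginPlay it takes initiative and damage from SaplingInfos, registers on its tile and adds tile HP.
; FindTarget sphere-traces for enemy-tagged tiles, then selects one using tag priority and squared distance.
; Fire launches a projectile timed to TurnTime, while Attack applies damage immediately, without waiting for impact.
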(event `self.ReceiveBeginPlay`
  (bind _linkedtile_0 (`self.LinkedTile_0`))
  (bind (_sapling _turntogrowth _initiative _overviewtext _tags _canattack_ _damage) (break `/Game/_Main/TCG/Cards/Data/S_Saplings` (`self.SaplingInfos`)))
  (`parent.ReceiveBeginPlay`)
  (set `self.Priority` _initiative)
  (set `self.Damage` _damage)
  (set `/Game/_Main/Level/LevelDesignElement/BP_TileBase.SaplingBuilding` self _linkedtile_0)
  (`/Game/_Main/Level/LevelDesignElement/BP_TileBase.Update SaplingType` _linkedtile_0)
  (`/Game/_Main/Level/LevelDesignElement/BP_TileBase.Add HPs` _linkedtile_0 3))

(event `/Game/_Main/BPI_EndPlayerTurn.Execute Player Turn`
  (bind _target (`self.FindTarget`))
  (`/Engine/EditorBlueprintResources/StandardMacros.IsValid` _target
    (:`Is Valid`
      (`self.Fire` _target)
      (`self.Attack` _target))
    (:`Is Not Valid`
      (`KismetSystemLibrary.PrintString` "NO TARGET FOUND (PC)"))))

(fn `Attack`
  (params (Target :type "/Game/_Main/Level/LevelDesignElement/BP_TileBase Object Reference"))
  (bind _gameplaytags (`/Game/_Main/Level/LevelDesignElement/BP_TileBase.GameplayTags` Target))
  (bind _enemyminion (`/Game/_Main/Level/LevelDesignElement/BP_TileBase.EnemyMinion` Target))
  (bind _lumberjackbuilding (`/Game/_Main/Level/LevelDesignElement/BP_TileBase.LumberJackBuilding` Target))
  (`/Engine/EditorBlueprintResources/StandardMacros.IsValid` Target
    (:`Is Valid`
      (if (`BlueprintGameplayTagLibrary.HasTag` _gameplaytags (struct :`TagName` "Ennemi.Minion"))
        (`/Engine/EditorBlueprintResources/StandardMacros.IsValid` _enemyminion
          (:`Is Valid`
            (`GameplayStatics.ApplyDamage` _enemyminion (`KismetMathLibrary.Conv_IntToDouble` (`self.Damage`)) null self)))
        (elif (`BlueprintGameplayTagLibrary.HasTag` _gameplaytags (struct :`TagName` "Ennemi.Building"))
          (`/Engine/EditorBlueprintResources/StandardMacros.IsValid` (`/Game/_Main/Level/LevelDesignElement/BP_TileBase.TileTypeVisual` Target)
            (:`Is Valid`
              (`GameplayStatics.ApplyDamage` _lumberjackbuilding (`KismetMathLibrary.Conv_IntToDouble` (`self.Damage`)) null self)
              (`KismetSystemLibrary.PrintString` (`KismetStringLibrary.Concat_StrStr` "Plant ATTACK : " (`KismetSystemLibrary.GetDisplayName` _lumberjackbuilding))))))))))

(fn `FindTarget`
  (returns (Target :type "/Game/_Main/Level/LevelDesignElement/BP_TileBase Object Reference"))
  (locals (PotentialTargets :type "Array of /Game/_Main/Level/LevelDesignElement/BP_TileBase Object Reference") (BestTarget :type "/Game/_Main/Level/LevelDesignElement/BP_TileBase Object Reference") (BestDistance :type "Float (double-precision)") (BestTargetPriority :type Integer) (BestTagPriority :type Integer) (BestGameplayTag :type "GameplayTag Structure"))
  (bind _besttagpriority (`local.BestTagPriority`))
  (bind _besttarget (`local.BestTarget`))
  (bind _potentialtargets (`local.PotentialTargets`))
  (bind _returnvalue (`self.K2_GetActorLocation` (`self.LinkedTile_0`)))
  (`|ExecutionSequence`
    (:`then_0`
      (bind _outhits (`KismetSystemLibrary.SphereTraceMultiForObjects` :`Start` _returnvalue :`End` _returnvalue :`Radius` (`KismetMathLibrary.Conv_IntToDouble` (`.RangeMax_40_3ACA23034E250E9CBD201D9D1F74DF94` (break `/Game/_Main/TCG/Cards/Data/S_Saplings` (`self.SaplingInfos`)))) :`ObjectTypes` (`|MakeArray` "ObjectTypeQuery7" :!type "EObjectTypeQuery Enum") :`DrawDebugType` "ForDuration"))
      (for _array_element _outhits
        (bind _asbp_tile_base (cast `/Game/_Main/Level/LevelDesignElement/BP_TileBase` (`.HitActor` (`GameplayStatics.BreakHitResult` _array_element))))
        (if (`BlueprintGameplayTagLibrary.HasTag` (`/Game/_Main/Level/LevelDesignElement/BP_TileBase.GameplayTags` _asbp_tile_base) (struct :`TagName` "Ennemi"))
          (`KismetArrayLibrary.Array_Add` (`local.PotentialTargets`) _asbp_tile_base))))
    (:`then_1`
      (set `local.BestGameplayTag` (struct))
      (set `local.BestTagPriority` 999)
      (set `local.BestTargetPriority` 999)
      (set `local.BestDistance` 9999999999.0)
      (set `local.BestTarget` null)
      (if (`KismetArrayLibrary.Array_IsNotEmpty` _potentialtargets)
        (for _array_element_2 _potentialtargets
          (bind _returnvalue_2 (`KismetMathLibrary.Vector_DistanceSquared` (`self.K2_GetActorLocation` _array_element_2) (`self.K2_GetActorLocation` (`self.LinkedTile_0`))))
          (if (< _returnvalue_2 (`local.BestDistance`))
            (for _array_element_3 (`BlueprintGameplayTagLibrary.BreakGameplayTagContainer` (`/Game/_Main/Level/LevelDesignElement/BP_TileBase.GameplayTags` _array_element_2))
              (bind (_value _returnvalue_3) (`BlueprintMapLibrary.Map_Find` (`self.TargetPriority`) _array_element_3))
              (if (and _returnvalue_3 (< _value (`local.BestTagPriority`)))
                (set `local.BestTagPriority` _value)
                (set `local.BestGameplayTag` _array_element_3)))
            (if (< _besttagpriority (`local.BestTargetPriority`))
              (set `local.BestTargetPriority` _besttagpriority)
              (set `local.BestDistance` _returnvalue_2)
              (set `local.BestTarget` _array_element_2))))
        (`/Engine/EditorBlueprintResources/StandardMacros.IsValid` _besttarget
          (:`Is Valid`
            (return _besttarget)))))))

(fn `Fire`
  (params (Target :type "/Game/_Main/Level/LevelDesignElement/BP_TileBase Object Reference"))
  (`/Engine/EditorBlueprintResources/StandardMacros.IsValid` Target
    (:`Is Valid`
      (`|SpawnActorFromClass` "/Game/_Main/Actors/Saplings/Projectile/BP_BaseProjectile.BP_BaseProjectile_C" (`self.GetTransform`) "Undefined" "MultiplyWithRoot" null (`self.K2_GetActorLocation`) (`self.K2_GetActorLocation` Target) (`self.TurnTime`) null))))

(fn `UserConstructionScript`)