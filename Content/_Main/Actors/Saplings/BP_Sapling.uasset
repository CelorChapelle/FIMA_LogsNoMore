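; BP_Sapling is a turn-based sapling actor that grows into another actor on its linked tile after a set number of player turns.
; BeginPlay copies the countdown from SaplingToGrowth, and each ExecutePlayerTurn decrements it.
; At zero, it spawns that struct's Sapling class at the tile, passing on tile and growth info, then destroys itself if the spawn succeeds.
; It reports its Priority to the turn system with zero turn time.
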(event `self.ReceiveBeginPlay`
  (`parent.ReceiveBeginPlay`)
  (set `self.TurnToGrowth` (`.TurnToGrowth_52_F77DDCF5459E0B7EC3432E9CD936BE11` (break `/Game/_Main/TCG/Cards/Data/S_Saplings` (`self.SaplingToGrowth`)))))

(event `/Game/_Main/BPI_EndPlayerTurn.Execute Player Turn`
  (bind _linkedtile_0 (`self.LinkedTile_0`))
  (set `self.TurnToGrowth` (- (`self.TurnToGrowth`) 1))
  (if (<= (`self.TurnToGrowth`) 0)
    (bind _returnvalue (`|SpawnActorFromClass` (`.Sapling_71_F3CF79F245E4D1D8FDA7F9B265CE39ED` (break `/Game/_Main/TCG/Cards/Data/S_Saplings` (`self.SaplingToGrowth`))) (`self.GetTransform` _linkedtile_0) "Undefined" "MultiplyWithRoot" null _linkedtile_0 (`self.SaplingToGrowth`) null null null null))
    (`/Engine/EditorBlueprintResources/StandardMacros.IsValid` _returnvalue
      (:`Is Valid`
        (`self.K2_DestroyActor`)))))

(fn `GetPlayerTurnPriority`
  (returns (Priority :type Integer) (TurnTime :type "Float (double-precision)"))
  (return (`self.Priority`) 0.0))

(fn `UserConstructionScript`
  (`parent.UserConstructionScript`))