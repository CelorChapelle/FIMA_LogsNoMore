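; Base lumberjack enemy for a turn-based tile game that seeks out and attacks forest tiles.
; Each action sphere-traces for the nearest forest, or follows a looping patrol offset list if none is found.
; Navigation paths are snapped to the grid to guide greedy four-way steps avoiding mountains, occupied tiles and backtracking.
; It maintains tile occupancy, hides under fog, and on death notifies its linked building and killer.
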(event `self.ReceiveBeginPlay`
  (set `self.Map Manager` (`/Game/_Main/BP_PlayerController.Map Manager` (`/Game/_Main/Level/LevelDesignElement/BP_TileBase.Player Controller` (`self.CurrentTile`))))
  (set `self.PreviousPatrolTarget` (`/Game/_Main/Level/LevelDesignElement/BP_TileBase.Coords` (`self.CurrentTile`)))
  (set `self.LastTile` (`self.CurrentTile`)))

(event `self.ReceiveTick`
  (params (DeltaSeconds :type "Float (single-precision)"))
  (for _array_element (`self.Path Points`)
    (`KismetSystemLibrary.SphereTraceSingle` :`Start` _array_element :`End` (+ _array_element (0.0 0.0 500.0)) :`Radius` 50.0 :`TraceChannel` "TraceTypeQuery1" :`DrawDebugType` "ForOneFrame")))

(event `/Game/_Main/BPI_EnemiTurn.Execute Enemi Turn`
  (set `self.CurrentAction` 0)
  (`self.ExecuteNextAction`))

(event `ExecuteNextAction`
  (bind _visible_ (`self.Visible?`))
  (if (< (`self.CurrentAction`) (`self.Movement`))
    (`self.ExecuteAIAction` (`self.CurrentTile`) (`self.Range`))
    (if _visible_
      (`KismetSystemLibrary.Delay` (/ (`self.TurnDuration`) (`self.Movement`))))
    (set `self.CurrentAction` (+ (`self.CurrentAction`) 1))
    (`self.ExecuteNextAction`)))

(event `self.ReceiveAnyDamage`
  (params (Damage :type "Float (single-precision)") (DamageType :type "DamageType Object Reference") (InstigatedBy :type "Controller Object Reference") (DamageCauser :type "Actor Object Reference"))
  (`self.TakeDamage` Damage DamageCauser))

(fn `Attack`
  (params (Target :type "/Game/_Main/Level/LevelDesignElement/BP_TileBase Object Reference"))
  (locals (CurrentDamage :type Integer))
  (`GameplayStatics.ApplyDamage` (`local.Target`) (`KismetMathLibrary.Conv_IntToDouble` (`self.Damage`)) null self))

(fn `ExecuteAIAction`
  (params (SourceRadius :type "/Game/_Main/Level/LevelDesignElement/BP_TileBase Object Reference") (Radius :type "Float (double-precision)"))
  (locals (L_BestTarget :type "/Game/_Main/Level/LevelDesignElement/BP_TileBase Object Reference") (L_TileToMooveOn :type "/Game/_Main/Level/LevelDesignElement/BP_TileBase Object Reference") (`Can'tWalkOn` :type "GameplayTagContainer Structure"))
  (bind (_output_x _output_y) (`KismetMathLibrary.BreakVector` (`|GetArrayItem` (`self.Path Points`) 1)))
  (bind _returnvalue (+ (* (`|GetArrayItem` (`self.PatrolTargets`) (`self.PatrolStep`)) (100.0 100.0)) (`self.PreviousPatrolTarget`)))
  (bind _target (`self.FindBestTarget` (`self.CurrentTile`) Radius))
  (`/Engine/EditorBlueprintResources/StandardMacros.IsValid` _target
    (:`Is Valid`
      (set `local.L_BestTarget` _target)
      (`SceneComponent.SetVisibility` (`self.BP_Alert`) true true)
      (bind _returnvalue_2 (`NavigationSystemV1.FindPathToActorSynchronously` (`self.K2_GetActorLocation`) (`local.L_BestTarget`) 50.0 null null))
      (bind _output_get (set `self.Path Points` (`NavigationPath.PathPoints` _returnvalue_2)))
      (if (`KismetArrayLibrary.Array_IsValidIndex` _output_get 1)
        (bind _tiletomooveon (`self.FindBestDirection` (`local.L_BestTarget`) (`KismetMathLibrary.MakeVector2D` (`KismetMathLibrary.GridSnap_Float` _output_x 100.0) (`KismetMathLibrary.GridSnap_Float` _output_y 100.0)) (`self.LastTile`)))
        (bind _gameplaytags (`/Game/_Main/Level/LevelDesignElement/BP_TileBase.GameplayTags` _tiletomooveon))
        (if (not (or (`BlueprintGameplayTagLibrary.HasTag` _gameplaytags (struct :`TagName` "Tile.Type.Forest") true) (`BlueprintGameplayTagLibrary.HasTag` _gameplaytags (struct :`TagName` "Tile.Type.OriginForest") true)))
          (if (not (== (`local.L_BestTarget`) _tiletomooveon))
            (`self.UpdateLumberJackPosition` _tiletomooveon)
            (else
              (`self.Attack` _tiletomooveon :!label _label)
              (`KismetSystemLibrary.PrintString` "Attack")))
          (else
            (goto _label)))
        (else
          (`KismetSystemLibrary.PrintString` "No Target" true true (struct :`R` 1.0 :`G` 0.340007 :`B` 0.40938 :`A` 1.0)))))
    (:`Is Not Valid`
      (`self.Patrol` _returnvalue)
      (`SceneComponent.SetVisibility` (`self.BP_Alert`) false true)
      (if (== _returnvalue (`/Game/_Main/Level/LevelDesignElement/BP_TileBase.Coords` (`self.CurrentTile`)))
        (set `self.PatrolStep` (+ (`self.PatrolStep`) 1))
        (if (== (`self.PatrolStep`) 13)
          (set `self.PatrolStep` 0))))))

(fn `FindBestDirection`
  (params (Target :type "/Game/_Main/Level/LevelDesignElement/BP_TileBase Object Reference") (NextPointCoords :type "Vector2D Structure") (LastTile :type "/Game/_Main/Level/LevelDesignElement/BP_TileBase Object Reference"))
  (returns (TileToMooveOn :type "/Game/_Main/Level/LevelDesignElement/BP_TileBase Object Reference"))
  (locals (BestTile :type "/Game/_Main/Level/LevelDesignElement/BP_TileBase Object Reference") (BestDistance :type "Float (double-precision)") (`Can'tWalkOn` :type "GameplayTagContainer Structure" :default (struct :`GameplayTags` (struct :`(TagName` "Tile.Type.Mountain") :`(TagName` "Ennemi.Minion.Renfort") :`(TagName` "Ennemi.Minion.LostLumberJack") :`(TagName` "Ennemi.Minion.ArcherLumberJack") :`(TagName` "Ennemi.Minion.LumberJack")))))
  (bind _besttile (`local.BestTile`))
  (bind (_nextpointcoords_x _nextpointcoords_y) (`KismetMathLibrary.BreakVector2D` (`local.NextPointCoords`)))
  (bind _currenttile (`self.CurrentTile`))
  (bind _coords (`/Game/_Main/Level/LevelDesignElement/BP_TileBase.Coords` (`self.CurrentTile`)))
  (bind _tilecoords (`/Game/_Main/BP_MapManager.TileCoords` (`self.Map Manager`)))
  (`KismetSystemLibrary.PrintString` (`KismetSystemLibrary.GetDisplayName` LastTile))
  (set `local.BestTile` null)
  (set `local.BestDistance` 9999999.0)
  (for _array_element (`|MakeArray` (`BlueprintMapLibrary.Map_Find` _tilecoords (+ _coords (100.0 0.0))) (`BlueprintMapLibrary.Map_Find` _tilecoords (+ _coords (0.0 100.0))) (`BlueprintMapLibrary.Map_Find` _tilecoords (+ _coords (-100.0 0.0))) (`BlueprintMapLibrary.Map_Find` _tilecoords (+ _coords (0.0 -100.0))))
    (`/Engine/EditorBlueprintResources/StandardMacros.IsValid` _array_element
      (:`Is Valid`
        (if (not (`BlueprintGameplayTagLibrary.HasTag` (`/Game/_Main/Level/LevelDesignElement/BP_TileBase.GameplayTags` _array_element) (struct :`TagName` "Tile.Type.Mountain") true))
          (bind (_coords_x _coords_y) (`KismetMathLibrary.BreakVector2D` (`/Game/_Main/Level/LevelDesignElement/BP_TileBase.Coords` _array_element)))
          (bind _returnvalue (+ (`KismetMathLibrary.Abs` (- _nextpointcoords_x _coords_x)) (`KismetMathLibrary.Abs` (- _nextpointcoords_y _coords_y))))
          (if (< _returnvalue (`local.BestDistance`))
            (if (`KismetSystemLibrary.IsValid` (`/Game/_Main/Level/LevelDesignElement/BP_TileBase.EnemyMinion` _array_element))
              _
              (elif (!= _array_element (`local.LastTile`))
                (set `local.BestTile` _array_element)
                (set `local.BestDistance` _returnvalue))))))))
  (`/Engine/EditorBlueprintResources/StandardMacros.IsValid` _besttile
    (:`Is Valid`
      (if (== _besttile _currenttile)
        _
        (else
          (return _besttile))))
    (:`Is Not Valid`
      _))
  (`KismetSystemLibrary.PrintString` "Do Not moove")
  (return _currenttile))

(fn `FindBestTarget`
  (params (RadiusSource :type "/Game/_Main/Level/LevelDesignElement/BP_TileBase Object Reference") (Radius :type "Float (double-precision)"))
  (returns (Target :type "/Game/_Main/Level/LevelDesignElement/BP_TileBase Object Reference") (TargetGameplayTag :type "GameplayTag Structure"))
  (locals (PotentalsTargets :type "Array of /Game/_Main/Level/LevelDesignElement/BP_TileBase Object Reference") (BestGameplayTag :type "GameplayTag Structure") (BestTagPriority :type Integer) (BestTargetPriority :type Integer) (BestDistance :type "Float (double-precision)") (BestTarget :type "/Game/_Main/Level/LevelDesignElement/BP_TileBase Object Reference"))
  (bind _returnvalue (`self.K2_GetActorLocation` RadiusSource))
  (bind _besttarget (`local.BestTarget`))
  (bind _potentalstargets (`local.PotentalsTargets`))
  (`|ExecutionSequence`
    (:`then_0`
      (bind (_outhits _returnvalue_2) (`KismetSystemLibrary.SphereTraceMultiForObjects` :`Start` _returnvalue :`End` _returnvalue :`Radius` (`self.Range`) :`ObjectTypes` (`|MakeArray` "ObjectTypeQuery7" :!type "EObjectTypeQuery Enum") :`TraceColor` (struct :`R` 1.0 :`G` 0.038824 :`B` 0.840837 :`A` 1.0) :`TraceHitColor` (struct :`G` 0.054298 :`B` 1.0 :`A` 1.0)))
      (if _returnvalue_2
        (for _array_element _outhits
          (bind _asbp_tile_base (cast `/Game/_Main/Level/LevelDesignElement/BP_TileBase` (`.HitActor` (`GameplayStatics.BreakHitResult` _array_element))))
          (if (`BlueprintGameplayTagLibrary.HasTag` (`/Game/_Main/Level/LevelDesignElement/BP_TileBase.GameplayTags` _asbp_tile_base) (struct :`TagName` "Tile.Type.Forest") true)
            (`KismetArrayLibrary.Array_Add` (`local.PotentalsTargets`) _asbp_tile_base)))))
    (:`then_1`
      (set `self.PrintStringTarget` null)
      (set `local.BestGameplayTag` (struct))
      (set `local.BestTagPriority` 999)
      (set `local.BestTargetPriority` 999)
      (set `local.BestDistance` 9999999999.0)
      (set `local.BestTarget` null)
      (if (`KismetArrayLibrary.Array_IsNotEmpty` _potentalstargets)
        (for _array_element_2 _potentalstargets
          (bind _returnvalue_3 (`KismetMathLibrary.Vector_DistanceSquared` (`self.K2_GetActorLocation` _array_element_2) (`self.K2_GetActorLocation` (`self.CurrentTile`))))
          (if (< _returnvalue_3 (`local.BestDistance`))
            (set `local.BestDistance` _returnvalue_3)
            (set `local.BestTarget` _array_element_2)))
        (set `self.PrintStringTarget` _besttarget)
        (return _besttarget (`local.BestGameplayTag`))))))

(fn `GetEnemiTurnPriority`
  (returns (Priority :type Integer) (ActionDuration :type "Float (double-precision)") (Enemy :type "Actor Object Reference"))
  (return (`self.Priority`) (`self.TurnDuration`) self))

(fn `Patrol`
  (params (Target :type "Vector2D Structure"))
  (bind _value (`BlueprintMapLibrary.Map_Find` (`/Game/_Main/BP_MapManager.TileCoords` (`self.Map Manager`)) Target))
  (bind _tiletomooveon (`self.FindBestDirection` _value (`/Game/_Main/Level/LevelDesignElement/BP_TileBase.Coords` _value) (`self.LastTile`)))
  (`self.UpdateLumberJackPosition` _tiletomooveon))

(fn `TakeDamage`
  (params (Damage :type "Float (double-precision)") (DamageCauser :type "Actor Object Reference"))
  (bind _linkedbuilding (`self.LinkedBuilding`))
  (bind _lastdamagecauser (`self.LastDamageCauser`))
  (bind _currenttile (`self.CurrentTile`))
  (set `self.LastDamageCauser` DamageCauser)
  (set `self.HP` (`KismetMathLibrary.Clamp` (- (`self.HP`) Damage) 0 5000))
  (if (== (`self.HP`) 0)
    (set `/Game/_Main/Level/LevelDesignElement/BP_TileBase.EnemyMinion` null _currenttile)
    (`BlueprintGameplayTagLibrary.RemoveGameplayTag` (`/Game/_Main/Level/LevelDesignElement/BP_TileBase.GameplayTags` _currenttile) (`self.GameplayTag`))
    (`/Engine/EditorBlueprintResources/StandardMacros.IsValid` _linkedbuilding
      (:`Is Valid`
        (message `/Game/_Main/BPI_EnemiTurn.UpdateNumberOfUnits` _linkedbuilding))
      (:`Is Not Valid`
        _))
    (`KismetSystemLibrary.PrintString` "LumberJackDead" true true (struct :`R` 0.090275 :`G` 0.257899 :`B` 1.0 :`A` 1.0) 4.0)
    (`/Engine/EditorBlueprintResources/StandardMacros.IsValid` _lastdamagecauser
      (:`Is Valid`
        (if (`KismetSystemLibrary.DoesImplementInterface` _lastdamagecauser "/Game/_Main/BPI_OnKill.BPI_OnKill_C")
          (message `/Game/_Main/BPI_OnKill.OnKill` _lastdamagecauser self)))
      (:`Is Not Valid`
        _))
    (`self.K2_DestroyActor`)))

(fn `UpdateLumberJackPosition`
  (params (TileToMooveOn :type "/Game/_Main/Level/LevelDesignElement/BP_TileBase Object Reference"))
  (bind _currenttile (`self.CurrentTile`))
  (set `self.LastTile` (`self.CurrentTile`))
  (`self.K2_SetActorLocation` (`self.K2_GetActorLocation` TileToMooveOn))
  (set `/Game/_Main/Level/LevelDesignElement/BP_TileBase.EnemyMinion` null _currenttile)
  (`BlueprintGameplayTagLibrary.RemoveGameplayTag` (`/Game/_Main/Level/LevelDesignElement/BP_TileBase.GameplayTags` _currenttile) (`self.GameplayTag`))
  (bind _output_get (set `self.CurrentTile` TileToMooveOn))
  (set `/Game/_Main/Level/LevelDesignElement/BP_TileBase.EnemyMinion` self _output_get)
  (`BlueprintGameplayTagLibrary.AddGameplayTag` (`/Game/_Main/Level/LevelDesignElement/BP_TileBase.GameplayTags` _output_get) (`self.GameplayTag`)))

(fn `UserConstructionScript`)

(fn `Visible?`
  (returns (`Visible?` :type Boolean))
  (if (`BlueprintGameplayTagLibrary.HasTag` (`/Game/_Main/Level/LevelDesignElement/BP_TileBase.GameplayTags` (`self.CurrentTile`)) (struct :`TagName` "Tile.State.Fogged") true)
    (`self.SetActorHiddenInGame` true)
    (return true)
    (else
      (`self.SetActorHiddenInGame` false)
      (return false))))