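; Lumberjack Palladin enemy, a child Blueprint that inherits its behavior from a parent enemy class and adjusts its AI targeting.
; FindBestTarget runs the parent search with a zero radius and falls back to the MapManager's origin tile when no valid target is found.
; ExecuteAIAction also forwards to the parent with a zero radius, ignoring the radius passed in; the event graph holds only disabled stubs.
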(fn `ExecuteAIAction`
  (params (SourceRadius :type "/Game/_Main/Level/LevelDesignElement/BP_TileBase Object Reference") (Radius :type "Float (double-precision)"))
  (`parent.ExecuteAIAction` null 0.0))

(fn `FindBestTarget`
  (params (RadiusSource :type "/Game/_Main/Level/LevelDesignElement/BP_TileBase Object Reference") (Radius :type "Float (double-precision)"))
  (returns (Target :type "/Game/_Main/Level/LevelDesignElement/BP_TileBase Object Reference") (TargetGameplayTag :type "GameplayTag Structure"))
  (bind _target (`parent.FindBestTarget` RadiusSource 0.0))
  (`/Engine/EditorBlueprintResources/StandardMacros.IsValid` _target
    (:`Is Valid`
      (return _target))
    (:`Is Not Valid`
      (return (`/Game/_Main/BP_MapManager.OriginTile` (`self.Map Manager`))))))

(fn `UserConstructionScript`
  (`parent.UserConstructionScript`))