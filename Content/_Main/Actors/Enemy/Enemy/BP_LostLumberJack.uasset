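; Lost lumberjack enemy that patrols the tile grid by wandering between neighboring tiles.
; Patrol gathers the current tile's neighbors, excluding mountain-tagged tiles and LastTile, then picks one at random.
; It calls UpdateLumberJackPosition only if that tile holds no enemy minion, with no retry otherwise.
; An unconnected sphere-trace variant for picking destinations within Range remains in Patrol but never runs.
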(event `self.ReceiveBeginPlay`
  (`parent.ReceiveBeginPlay`)
  (set `self.PositionToGo` (`/Game/_Main/Level/LevelDesignElement/BP_TileBase.Coords` (`self.CurrentTile`)))
  (set `self.LastTile` (`self.CurrentTile`)))

(event `self.ReceiveAnyDamage`
  (params (Damage :type "Float (single-precision)") (DamageType :type "DamageType Object Reference") (InstigatedBy :type "Controller Object Reference") (DamageCauser :type "Actor Object Reference"))
  (`parent.ReceiveAnyDamage` Damage DamageType InstigatedBy DamageCauser))

(fn `Patrol`
  (params (Target :type "Vector2D Structure"))
  (locals (PotentielsTargets :type "Array of /Game/_Main/Level/LevelDesignElement/BP_TileBase Object Reference") (TemporaryTarget :type "/Game/_Main/Level/LevelDesignElement/BP_TileBase Object Reference"))
  (bind _potentielstargets (`local.PotentielsTargets`))
  (`KismetArrayLibrary.Array_Clear` (`local.PotentielsTargets`))
  (for _array_element (`/Game/_Main/Level/LevelDesignElement/BP_TileBase.Voisins` (`self.CurrentTile`))
    (`/Engine/EditorBlueprintResources/StandardMacros.IsValid` _array_element
      (:`Is Valid`
        (if (not (`BlueprintGameplayTagLibrary.HasTag` (`/Game/_Main/Level/LevelDesignElement/BP_TileBase.GameplayTags` _array_element) (struct :`TagName` "Tile.Type.Mountain") true))
          (if (!= _array_element (`self.LastTile`))
            (`KismetArrayLibrary.Array_Add` (`local.PotentielsTargets`) _array_element))))))
  (bind _output_get (set `local.TemporaryTarget` (`|GetArrayItem` _potentielstargets (`KismetMathLibrary.RandomIntegerInRange` 0 (- (`KismetArrayLibrary.Array_Length` _potentielstargets) 1)))))
  (`/Engine/EditorBlueprintResources/StandardMacros.IsValid` (`/Game/_Main/Level/LevelDesignElement/BP_TileBase.EnemyMinion` _output_get)
    (:`Is Not Valid`
      (`/Engine/EditorBlueprintResources/StandardMacros.IsValid` _output_get
        (:`Is Valid`
          (`self.UpdateLumberJackPosition` (`local.TemporaryTarget`)))))))

(fn `UserConstructionScript`
  (`parent.UserConstructionScript`))