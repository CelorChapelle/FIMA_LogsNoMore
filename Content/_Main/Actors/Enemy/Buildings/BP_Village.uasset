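; BP_Village is an enemy building that spawns archers, walls and lumberjacks during the enemy turn.
; On its turn it runs forest detection and a wall spawn check, then calls the archer, wall and outside lumberjack spawn functions in sequence, none of which are defined in this graph.
; It reports itself with zero turn priority and zero action duration, and defers BeginPlay and unit count updates to its parent.
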(event `self.ReceiveBeginPlay`
  (`parent.ReceiveBeginPlay`))

(event `/Game/_Main/BPI_EnemiTurn.Execute Enemi Turn`
  (`self.ForestDetection`)
  (`self.CanSpawnWall?`)
  (`self.SpawnArcher`)
  (`self.SpawnWall`)
  (`self.SpawnLumberJackOutside`))

(event `/Game/_Main/BPI_EnemiTurn.UpdateNumberOfUnits`
  (`parent.UpdateNumberOfUnits`))

(fn `GetEnemiTurnPriority`
  (returns (Priority :type Integer) (ActionDuration :type "Float (double-precision)") (Enemy :type "Actor Object Reference"))
  (return 0 0.0 self))

(fn `UserConstructionScript`)