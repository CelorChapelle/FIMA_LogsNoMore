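; BP_City is an enemy city building whose destruction wins the game for the player.
; On its enemy turn it runs forest detection, then calls spawns for archers and lumberjack or paladin units.
; It reports itself to the turn system with zero priority and duration.
; Damage reduces its clamped HP, and at zero it triggers Victory on the player controller and destroys itself.
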(event `self.ReceiveBeginPlay`
  (`parent.ReceiveBeginPlay`))

(event `self.Execute Enemi Turn`
  (`self.ForestDetection`)
  (`self.SpawnArcher`)
  (`self.SpawnLumberJackPalladinOutside`))

(event `self.UpdateNumberOfUnits`
  (`parent.UpdateNumberOfUnits`))

(fn `GetEnemiTurnPriority`
  (returns (Priority :type Integer) (ActionDuration :type "Float (double-precision)") (Enemy :type "Actor Object Reference"))
  (return 0 0.0 self))

(fn `TakeDamage`
  (params (Damage :type "Float (double-precision)"))
  (bind _hp (`self.Hp`))
  (set `self.Hp` (`KismetMathLibrary.FClamp` (- _hp Damage) 0.0 50.0))
  (if (== _hp 0.0)
    (`/Game/_Main/BP_PlayerController.Victory !` (`self.Player Controller`))
    (`self.K2_DestroyActor`)))

(fn `UserConstructionScript`)