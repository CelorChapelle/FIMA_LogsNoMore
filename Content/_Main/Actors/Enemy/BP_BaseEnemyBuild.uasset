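; Base enemy building on the tile map, with turn priority, lumberjack and archer spawning, and wall placement.
; Its turn runs ForestDetection, which sets CanSpawn when a forest or forest-adjacent tile lies within AlertRadius.
; Spawn helpers, not called here, use that flag, unit caps, turn counters and coordinate offsets from the parent tile.
; At zero HP it clears its tile tag and destroys itself, leaving ruins only through the AnyDamage path.
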(event `self.ReceiveBeginPlay`)

(event `/Game/_Main/BPI_EnemiTurn.Execute Enemi Turn`
  (`self.ForestDetection`))

(event `/Game/_Main/BPI_EnemiTurn.UpdateNumberOfUnits`
  (bind _output_get (set `self.ActualsUnits` (- (`self.ActualsUnits`) 1))))

(event `self.ReceiveAnyDamage`
  (params (Damage :type "Float (single-precision)") (DamageType :type "DamageType Object Reference") (InstigatedBy :type "Controller Object Reference") (DamageCauser :type "Actor Object Reference"))
  (bind _hp (`self.Hp`))
  (bind _parenttile (`self.ParentTile`))
  (set `self.Hp` (`KismetMathLibrary.FClamp` (- _hp Damage) 0.0 50.0))
  (if (== _hp 0.0)
    (`BlueprintGameplayTagLibrary.RemoveGameplayTag` (`/Game/_Main/Level/LevelDesignElement/BP_TileBase.GameplayTags` _parenttile) (`self.GameplayTag`))
    (`|SpawnActorFromClass` "/Game/_Main/Actors/BP_HumansRuins.BP_HumansRuins_C" (`self.GetTransform` _parenttile) "Undefined" "MultiplyWithRoot" null null null _parenttile null)
    (`self.K2_DestroyActor`)))

(fn `CanSpawnWall?`
  (if (`self.CanSpawn`)
    (bind _output_get (set `self.TurnToSpawnWall` (+ (`self.TurnToSpawnWall`) 1)))
    (if (== _output_get 2)
      _)))

(fn `Destroy&UpdateTileType`
  (bind _parenttile (`self.ParentTile`))
  (set `/Game/_Main/Level/LevelDesignElement/BP_TileBase.LumberJackBuilding` self _parenttile)
  (`/Game/_Main/BP_CardEffectManager.UpdateTileType` (`/Game/_Main/BP_PlayerController.CardEffectManager` (`/Game/_Main/Level/LevelDesignElement/BP_TileBase.Player Controller` _parenttile)) self _parenttile)
  (`/Game/_Main/Level/LevelDesignElement/BP_TileBase.UpdateTileandNeigboursAdjToForest` _parenttile)
  (`BlueprintGameplayTagLibrary.AddGameplayTag` (`/Game/_Main/Level/LevelDesignElement/BP_TileBase.GameplayTags` _parenttile) (struct :`TagName` "Tile.Type.Plain")))

(fn `FindPositionToSpawnUnit`
  (returns (`Tile to Spawn` :type "/Game/_Main/Level/LevelDesignElement/BP_TileBase Object Reference"))
  (locals (BasePositionToCheck :type "Array of Vector2D Structure") (Target :type "/Game/_Main/Level/LevelDesignElement/BP_TileBase Object Reference"))
  (bind _parenttile (`self.ParentTile`))
  (for _array_element (`local.BasePositionToCheck`)
    (bind _value (`BlueprintMapLibrary.Map_Find` (`/Game/_Main/BP_MapManager.TileCoords` (`/Game/_Main/BP_PlayerController.Map Manager` (`/Game/_Main/Level/LevelDesignElement/BP_TileBase.Player Controller` _parenttile))) (+ (* _array_element (100.0 100.0)) (`/Game/_Main/Level/LevelDesignElement/BP_TileBase.Coords` _parenttile))))
    (if (`KismetSystemLibrary.IsValid` (`/Game/_Main/Level/LevelDesignElement/BP_TileBase.EnemyMinion` _value))
      (set `local.Target` _value)
      (break)))
  (return (`local.Target`)))

(fn `ForestDetection`
  (bind _parenttile (`self.ParentTile`))
  (bind _alertradius (`self.AlertRadius`))
  (bind (_coords_x _coords_y) (`KismetMathLibrary.BreakVector2D` (`/Game/_Main/Level/LevelDesignElement/BP_TileBase.Coords` _parenttile)))
  (for _index (range (* _alertradius -1) (+ _alertradius 1))
    (for _index_2 (range (* _alertradius -1) (+ _alertradius 1))
      (bind _value (`BlueprintMapLibrary.Map_Find` (`/Game/_Main/BP_MapManager.TileCoords` (`/Game/_Main/BP_PlayerController.Map Manager` (`/Game/_Main/Level/LevelDesignElement/BP_TileBase.Player Controller` _parenttile))) (`KismetMathLibrary.MakeVector2D` (+ _coords_x (* _index 100)) (+ _coords_y (* _index_2 100)))))
      (`/Engine/EditorBlueprintResources/StandardMacros.IsValid` _value
        (:`Is Valid`
          (bind _gameplaytags (`/Game/_Main/Level/LevelDesignElement/BP_TileBase.GameplayTags` _value))
          (if (or (`BlueprintGameplayTagLibrary.HasTag` _gameplaytags (struct :`TagName` "Tile.State.AdjacentToForest") true) (`BlueprintGameplayTagLibrary.HasTag` _gameplaytags (struct :`TagName` "Tile.Type.Forest") true))
            (set `self.CanSpawn` true)))))))

(fn `GetEnemiTurnPriority`
  (returns (Priority :type Integer) (ActionDuration :type "Float (double-precision)"))
  (return (`self.TurnPriority`) (`self.TurnDuration`)))

(fn `SpawnArcher`
  (bind _parenttile (`self.ParentTile`))
  (bind _parenttile_2 (`self.ParentTile`))
  (if (and (not (`KismetSystemLibrary.IsValid` (`/Game/_Main/Level/LevelDesignElement/BP_TileBase.EnemyMinion` (`self.ParentTile`)))) (`self.CanSpawn`))
    (bind _output_get (set `self.TurnToRespawnCount` (+ (`self.TurnToRespawnCount`) 1)))
    (if (== (`self.TurnToRespawnArcher`) _output_get)
      (bind _returnvalue (`|SpawnActorFromClass` "/Game/_Main/Actors/Enemy/Enemy/BP_LumberJackArcher.BP_LumberJackArcher_C" (`self.GetTransform` _parenttile) "Undefined" "MultiplyWithRoot" null _parenttile null null null))
      (set `/Game/_Main/Level/LevelDesignElement/BP_TileBase.EnemyMinion` _returnvalue _parenttile_2)
      (`BlueprintGameplayTagLibrary.AddGameplayTag` (`/Game/_Main/Level/LevelDesignElement/BP_TileBase.GameplayTags` _parenttile_2) (`/Game/_Main/Actors/Enemy/BP_LumberJackBase.GameplayTag` _returnvalue))
      (set `self.TurnToRespawnCount` 0))))

(fn `SpawnLumberJackInside`
  (bind _parenttile (`self.ParentTile`))
  (bind _parenttile_2 (`self.ParentTile`))
  (bind _parenttile_3 (`self.ParentTile`))
  (if (and (< (`self.ActualsUnits`) (`self.MaxAliveUnits`)) (`self.CanSpawn`))
    (if (not (`KismetSystemLibrary.IsValid` (`/Game/_Main/Level/LevelDesignElement/BP_TileBase.EnemyMinion` (`self.ParentTile`))))
      (bind _returnvalue (`|SpawnActorFromClass` "/Game/_Main/Actors/Enemy/Enemy/BP_LumberJack.BP_LumberJack_C" (`self.GetTransform` _parenttile_3) "Undefined" "MultiplyWithRoot" null _parenttile_3 null self null))
      (set `self.ActualsUnits` (+ (`self.ActualsUnits`) 1))
      (set `/Game/_Main/Level/LevelDesignElement/BP_TileBase.EnemyMinion` _returnvalue _parenttile)
      (`BlueprintGameplayTagLibrary.AddGameplayTag` (`/Game/_Main/Level/LevelDesignElement/BP_TileBase.GameplayTags` _parenttile) (`/Game/_Main/Actors/Enemy/BP_LumberJackBase.GameplayTag` _returnvalue))
      (set `self.CanSpawn` false)
      (else
        (bind _tile_to_spawn (`self.FindPositionToSpawnUnit`))
        (`/Engine/EditorBlueprintResources/StandardMacros.IsValid` _tile_to_spawn
          (:`Is Valid`
            (bind _returnvalue_2 (`|SpawnActorFromClass` "/Game/_Main/Actors/Enemy/Enemy/BP_LumberJack.BP_LumberJack_C" (`self.GetTransform` _tile_to_spawn) "Undefined" "MultiplyWithRoot" null _tile_to_spawn null self null))
            (set `self.ActualsUnits` (+ (`self.ActualsUnits`) 1))
            (set `/Game/_Main/Level/LevelDesignElement/BP_TileBase.EnemyMinion` _returnvalue_2 _parenttile_2)
            (`BlueprintGameplayTagLibrary.AddGameplayTag` (`/Game/_Main/Level/LevelDesignElement/BP_TileBase.GameplayTags` _parenttile_2) (`/Game/_Main/Actors/Enemy/BP_LumberJackBase.GameplayTag` _returnvalue_2))
            (set `self.CanSpawn` false)))))))

(fn `SpawnLumberJackOutside`
  (bind _parenttile (`self.ParentTile`))
  (if (and (< (`self.ActualsUnits`) (`self.MaxAliveUnits`)) (`self.CanSpawn`))
    (bind _tile_to_spawn (`self.FindPositionToSpawnUnit`))
    (`/Engine/EditorBlueprintResources/StandardMacros.IsValid` _tile_to_spawn
      (:`Is Valid`
        (bind _returnvalue (`|SpawnActorFromClass` "/Game/_Main/Actors/Enemy/Enemy/BP_LumberJack.BP_LumberJack_C" (`self.GetTransform` _tile_to_spawn) "Undefined" "MultiplyWithRoot" null _tile_to_spawn null self null))
        (set `self.ActualsUnits` (+ (`self.ActualsUnits`) 1))
        (set `/Game/_Main/Level/LevelDesignElement/BP_TileBase.EnemyMinion` _returnvalue _parenttile)
        (`BlueprintGameplayTagLibrary.AddGameplayTag` (`/Game/_Main/Level/LevelDesignElement/BP_TileBase.GameplayTags` _parenttile) (`/Game/_Main/Actors/Enemy/BP_LumberJackBase.GameplayTag` _returnvalue))
        (set `self.CanSpawn` false)))))

(fn `SpawnWall`
  (locals (Coordinates :type "Array of Vector2D Structure") (CornerCoordinates :type "Array of Vector2D Structure") (Rotation :type "Float (double-precision)" :default -270.0) (Wallspawned :type Integer))
  (if (== (`self.TurnToSpawnWall`) 2)
    (for _array_element (`local.Coordinates`)
      (`KismetArrayLibrary.Array_Add` (`self.StraightWallCoords`) (+ (* _array_element (100.0 100.0)) (`/Game/_Main/Level/LevelDesignElement/BP_TileBase.Coords` (`self.ParentTile`)))))
    (for _array_element_2 (`local.CornerCoordinates`)
      (`KismetArrayLibrary.Array_Add` (`self.CornerWallCoords`) (+ (* _array_element_2 (100.0 100.0)) (`/Game/_Main/Level/LevelDesignElement/BP_TileBase.Coords` (`self.ParentTile`)))))
    (`|ExecutionSequence`
      (:`then_0`
        (for _array_element_3 (`self.StraightWallCoords`)
          (bind _output_get (set `local.Wallspawned` (+ (`local.Wallspawned`) 1)))
          (if (> _output_get 6)
            (bind _value (`BlueprintMapLibrary.Map_Find` (`/Game/_Main/BP_MapManager.TileCoords` (`/Game/_Main/BP_PlayerController.Map Manager` (`/Game/_Main/Level/LevelDesignElement/BP_TileBase.Player Controller` (`self.ParentTile`)))) _array_element_3))
            (bind _returnvalue (`self.GetTransform` _value))
            (`|SpawnActorFromClass` "/Game/_Main/Actors/Enemy/Buildings/BP_Wall1.BP_Wall1_C" _returnvalue "Undefined" "MultiplyWithRoot" null _value null null null null)
            (else
              (`|SpawnActorFromClass` "/Game/_Main/Actors/Enemy/Buildings/BP_Wall.BP_Wall_C" _returnvalue "Undefined" "MultiplyWithRoot" null _value null null null null)))))
      (:`then_1`
        (for _array_element_4 (`self.CornerWallCoords`)
          (bind _output_get_2 (set `local.Rotation` (+ 90.0 (`local.Rotation`))))
          (bind _value_2 (`BlueprintMapLibrary.Map_Find` (`/Game/_Main/BP_MapManager.TileCoords` (`/Game/_Main/BP_PlayerController.Map Manager` (`/Game/_Main/Level/LevelDesignElement/BP_TileBase.Player Controller` (`self.ParentTile`)))) _array_element_4))
          (bind _returnvalue_2 (`self.GetTransform` _value_2))
          (`|SpawnActorFromClass` "/Game/_Main/Actors/Enemy/Buildings/BP_WallCorner.BP_WallCorner_C" (`KismetMathLibrary.MakeTransform` (.location _returnvalue_2) (`KismetMathLibrary.MakeRotator` (.roll (.rotation _returnvalue_2)) (.pitch (.rotation _returnvalue_2)) _output_get_2) (.scale _returnvalue_2)) "Undefined" "MultiplyWithRoot" null _value_2 null null null null)))
      (:`then_2`
        (set `self.CanSpawnWall` false)))))

(fn `TakeDamage`
  (params (Damage :type "Float (double-precision)"))
  (bind _parenttile (`self.ParentTile`))
  (bind _hp (`self.Hp`))
  (set `self.Hp` (`KismetMathLibrary.FClamp` (- _hp Damage) 0.0 50.0))
  (if (== _hp 0.0)
    (`BlueprintGameplayTagLibrary.RemoveGameplayTag` (`/Game/_Main/Level/LevelDesignElement/BP_TileBase.GameplayTags` _parenttile) (`self.GameplayTag`))
    (set `/Game/_Main/Level/LevelDesignElement/BP_TileBase.LumberJackBuilding` null _parenttile)
    (`self.K2_DestroyActor`)))

(fn `UserConstructionScript`)