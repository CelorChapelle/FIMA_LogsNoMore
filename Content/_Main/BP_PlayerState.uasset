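; Player state for a deckbuilding card game, owning the deck and the draw, hand, discard, destroyed and reward piles.
; BeginPlay builds card instances from GameInstance row data and shuffles the draw pile, which DrawCard refills from discards.
; PlayCard checks mana, sends each tag/power pair to the controller's CardEffectManager, then discards or destroys exhaust cards.
; It also adds cards mid-game, discards hands with ephemeral handling, and feeds new cards and three-card rewards to the HUD.
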(event `self.ReceiveBeginPlay`
  (bind _asbp_game_instance (cast `/Game/_Main/BP_GameInstance` (`GameplayStatics.GetGameInstance`)))
  (set `self.GameInstance` _asbp_game_instance)
  (bind _asbp_player_controller (cast `/Game/_Main/BP_PlayerController` (`self.GetPlayerController`)))
  (set `self.Player Controller` _asbp_player_controller)
  (`self.CreateStartingDeck`)
  (`self.CreateDrawPile` (`self.Deck`))
  (`self.CreateRewadPile`))

(fn `AddCardToDeck`
  (params (RawName :type Name))
  (returns (CardInstance :type "/Game/_Main/TCG/Cards/Data/S_CardInstance Structure"))
  (bind (_days _hours _minutes _seconds) (`KismetMathLibrary.BreakTimespan2` (`KismetMathLibrary.GetTimeOfDay` (`KismetMathLibrary.Now`))))
  (bind _struct_carddata (`/Game/_Main/BP_GameInstance.GetCardData(RowName)` (`self.GameInstance`) RawName))
  (bind _returnvalue (`KismetArrayLibrary.Array_Add` (`self.Deck`) (make `/Game/_Main/TCG/Cards/Data/S_CardInstance` RawName (`.Cost_11_AE692AEF4D8F42A2B6FFF09A8B22CB33` (break `/Game/_Main/TCG/Cards/Data/S_CardData` _struct_carddata)) 0 (`KismetMathLibrary.FFloor` (* (+ (+ (* _days _hours) _seconds) (`KismetMathLibrary.RandomIntegerInRange` 1 200)) (`GameplayStatics.GetTimeSeconds`))) _struct_carddata)))
  (return (`|GetArrayItem` (`self.Deck`) _returnvalue)))

(fn `AddNewCardToDiscardPile`
  (params (RawName :type Name))
  (bind _cardinstance (`self.AddCardToDeck` RawName))
  (`self.DiscardCard` _cardinstance))

(fn `AddNewCardToHand`
  (params (CardInstanceToAdd :type "/Game/_Main/TCG/Cards/Data/S_CardInstance Structure"))
  (`KismetArrayLibrary.Array_Add` (`self.Hand`) CardInstanceToAdd)
  ; AddCardToHud
  (`/Game/_Main/TCG/Cards/Widget/WBP_HUD.AddNewCard` (`/Game/_Main/BP_PlayerController.HUD` (`self.Player Controller`)) CardInstanceToAdd))

(fn `AddNewCopieCardToHand`
  (params (CardInstanceToAdd :type "/Game/_Main/TCG/Cards/Data/S_CardInstance Structure"))
  (bind _cardinstance (`self.AddCardToDeck` (`.RowName_2_30A752C14B31894CEFDFC9A4099F3A23` (break `/Game/_Main/TCG/Cards/Data/S_CardInstance` CardInstanceToAdd))))
  (`KismetArrayLibrary.Array_Add` (`self.Hand`) _cardinstance))

(fn `CreateDrawPile`
  (params (Cards :type "Array of /Game/_Main/TCG/Cards/Data/S_CardInstance Structure"))
  (bind _drawpile (`self.DrawPile`))
  ; Clear la draw pile avant de piocher
  (`KismetArrayLibrary.Array_Clear` (`self.DrawPile`))
  (for _array_element Cards
    (`KismetArrayLibrary.Array_Add` _drawpile _array_element))
  (`KismetArrayLibrary.Array_Shuffle` _drawpile)
  (`KismetArrayLibrary.Array_Clear` (`self.DiscardPile`)))

(fn `CreateRewadPile`
  (for (_array_element _array_index) (`self.CardRewards`)
    (bind _struct_carddata (`/Game/_Main/BP_GameInstance.GetCardData(RowName)` (`self.GameInstance`) _array_element))
    (`KismetArrayLibrary.Array_Add` (`self.RewardPile`) (make `/Game/_Main/TCG/Cards/Data/S_CardInstance` _array_element (`.Cost_11_AE692AEF4D8F42A2B6FFF09A8B22CB33` (break `/Game/_Main/TCG/Cards/Data/S_CardData` _struct_carddata)) 0 (+ _array_index 1) _struct_carddata))))

(fn `CreateStartingDeck`
  (for (_array_element _array_index) (`self.StartingDeck`)
    (bind _struct_carddata (`/Game/_Main/BP_GameInstance.GetCardData(RowName)` (`self.GameInstance`) _array_element))
    (`KismetArrayLibrary.Array_Add` (`self.Deck`) (make `/Game/_Main/TCG/Cards/Data/S_CardInstance` _array_element (`.Cost_11_AE692AEF4D8F42A2B6FFF09A8B22CB33` (break `/Game/_Main/TCG/Cards/Data/S_CardData` _struct_carddata)) 0 (+ _array_index 1) _struct_carddata))))

(fn `DestroyCard`
  (params (CardToDestroy :type "/Game/_Main/TCG/Cards/Data/S_CardInstance Structure"))
  (`KismetArrayLibrary.Array_Add` (`self.DestroyedPile`) CardToDestroy)
  (`KismetArrayLibrary.Array_RemoveItem` (`self.Hand`) CardToDestroy)
  (`KismetArrayLibrary.Array_RemoveItem` (`self.Deck`) (make `/Game/_Main/TCG/Cards/Data/S_CardInstance` "None" 0 0 (`.InstanceID_9_BF7565DB44604819C773EFB60FE220DB` (break `/Game/_Main/TCG/Cards/Data/S_CardInstance` CardToDestroy)) (struct :`Type` "NewEnumerator0" :`InstigatorTag` "(NewEnumerator0)" :`Target` (struct) :`MandatoryTarget` (struct) :`SaplingToGrowth` "False"))))

(fn `DiscardCard`
  (params (CardToDiscard :type "/Game/_Main/TCG/Cards/Data/S_CardInstance Structure"))
  (`KismetArrayLibrary.Array_Add` (`self.DiscardPile`) CardToDiscard))

(fn `DiscardFromHandCard`
  (params (CardToDiscard :type "/Game/_Main/TCG/Cards/Data/S_CardInstance Structure"))
  (`KismetArrayLibrary.Array_Add` (`self.DiscardPile`) CardToDiscard)
  (`KismetArrayLibrary.Array_RemoveItem` (`self.Hand`) CardToDiscard))

(fn `DiscardFullHand`
  (locals (`IsEphemeral?` :type Boolean))
  (bind _hand (`self.Hand`))
  (for _array_element _hand
    (bind _keypin (`|MapForEach` (`.Tags_43_0CAC4B274E43B8305DBD73A4ABF2C1CF` (break `/Game/_Main/TCG/Cards/Data/S_CardData` (`.CardData_18_E97FEC6A494667101BBA969E8A2DCF93` (break `/Game/_Main/TCG/Cards/Data/S_CardInstance` _array_element)))))
      (:`then`
        (if (`|EnumEquality` _keypin "NewEnumerator13")
          (set `local.IsEphemeral?` true)))
      (:`CompletedPin`
        (if (`local.IsEphemeral?`)
          (`self.DestroyCard` _array_element)
          (else
            (`KismetArrayLibrary.Array_Add` (`self.DiscardPile`) _array_element))))))
  (`KismetArrayLibrary.Array_Clear` _hand)
  (return))

(fn `DrawCard`
  (params (CardsToDraw :type Integer :default 1))
  (bind _output (`|GetArrayItem` (`self.DrawPile`)))
  (bind (_playerstats_visibilityrange _playerstats_mana _playerstats_manaperturn _playerstats_tempovermana _playerstats_drawcardperturn _playerstats_maxhandsize) (break `/Game/_Main/Actors/Struct/S_PlayerStats` (`/Game/_Main/BP_PlayerController.PlayerStats` (`self.Player Controller`))))
  (for _ (range CardsToDraw)
    (if (and (`KismetArrayLibrary.Array_IsNotEmpty` (`self.DrawPile`)) (< (+ (`KismetArrayLibrary.Array_Length` (`self.Hand`)) 1) _playerstats_maxhandsize))
      (`KismetArrayLibrary.Array_Add` (`self.Hand`) _output :!label _label)
      ; AddCardToHud
      (`/Game/_Main/TCG/Cards/Widget/WBP_HUD.AddNewCard` (`/Game/_Main/BP_PlayerController.HUD` (`self.Player Controller`)) _output)
      (`KismetArrayLibrary.Array_Remove` (`self.DrawPile`))
      (else
        (`self.CreateDrawPile` (`self.DiscardPile`))
        (if (`KismetArrayLibrary.Array_IsNotEmpty` (`self.DrawPile`))
          (goto _label)
          (else
            (`KismetSystemLibrary.PrintString` "NoCardInDrawPile" true true (struct :`R` 1.0 :`G` 0.026958 :`A` 1.0) 4.0)))))))

(fn `PlayCard`
  (params (CardInstance :type "/Game/_Main/TCG/Cards/Data/S_CardInstance Structure") (Target :type "/Game/_Main/Level/LevelDesignElement/BP_TileBase Object Reference"))
  (bind (_rowname _currentcost _qualitylevel _instanceid _carddata) (break `/Game/_Main/TCG/Cards/Data/S_CardInstance` CardInstance))
  (bind _player_controller (`self.Player Controller`))
  (bind (_type _cost _instigatortag _tags _exhaust_ _text _target _mandatorytarget _saplingtogrowth) (break `/Game/_Main/TCG/Cards/Data/S_CardData` _carddata))
  (bind (_playerstats_visibilityrange _playerstats_mana) (break `/Game/_Main/Actors/Struct/S_PlayerStats` (`/Game/_Main/BP_PlayerController.PlayerStats` (`self.Player Controller`))))
  (if (>= _playerstats_mana _currentcost)
    (`/Game/_Main/BP_PlayerController.UpdateMana` _player_controller _currentcost)
    (bind (_keypin _valuepin) (`|MapForEach` _tags)
      (:`then`
        (`/Game/_Main/BP_CardEffectManager.PlayEffect` (`/Game/_Main/BP_PlayerController.CardEffectManager` (`self.Player Controller`)) (`local.Target`) _keypin _valuepin _saplingtogrowth))
      (:`CompletedPin`
        (if _exhaust_
          (`self.DestroyCard` CardInstance)
          (else
            (`self.DiscardFromHandCard` CardInstance)))))
    (else
      (`/Game/_Main/BP_PlayerController.UnplayCurrentCard` _player_controller))))

(fn `UpdateRewardCard`
  (if (and (`KismetArrayLibrary.Array_IsNotEmpty` (`self.RewardPile`)) (!= (`self.Multiple Reward`) 0))
    (`KismetArrayLibrary.Array_Shuffle` (`self.RewardPile`))
    ; AddCardToHud
    (`/Game/_Main/TCG/Cards/Widget/WBP_HUD.SetupNewReward` (`/Game/_Main/BP_PlayerController.HUD` (`self.Player Controller`)) (`|GetArrayItem` (`self.RewardPile`)) (`|GetArrayItem` (`self.RewardPile`) 1) (`|GetArrayItem` (`self.RewardPile`) 2))
    (else
      (`KismetSystemLibrary.PrintString` "No More REWARD" true true (struct :`R` 1.0 :`G` 0.026958 :`A` 1.0) 4.0))))

(fn `UserConstructionScript`)