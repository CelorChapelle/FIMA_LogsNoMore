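; Base grid tile that turns its designer-set type into gameplay tags and spawned visuals, buildings or forests, plus fog of war and tagged enemy minions.
; Gameplay tags drive its material.
; Forest tiles mark their four neighbours as forest-adjacent and clear fog within the player's visibility range by sphere trace.
; Damage consumes Protection, Shield, then forest HP; destroyed forest reverts to plain, and losing an origin forest ends the game.
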(event `self.ReceiveBeginPlay`
  (bind (_returnvalue_x _returnvalue_y) (`KismetMathLibrary.BreakVector` (`self.K2_GetActorLocation`)))
  (bind _gameplaytags (`self.GameplayTags`))
  (add `self.UpdateMaterial` (delegate `UpdateTileMaterial`))
  (bind _asbp_player_controller (cast `/Game/_Main/BP_PlayerController` (`GameplayStatics.GetPlayerController` 0)))
  (set `self.Player Controller` _asbp_player_controller)
  (`|ExecutionSequence`
    (:`then_0`
      (`PrimitiveComponent.SetMaterial` (`self.Cube`) 0 (`BlueprintMapLibrary.Map_Find` (`self.LDTool_MaterialID`) (`self.TileType`)))
      (switch `/Game/_Main/Level/LevelDesignElement/E_TileType` (`self.TileType`)
        (:`NewEnumerator7`
          (`BlueprintGameplayTagLibrary.AddGameplayTag` _gameplaytags (struct :`TagName` "Tile")))
        (:`NewEnumerator5`
          (`BlueprintGameplayTagLibrary.AddGameplayTag` _gameplaytags (struct :`TagName` "Tile.Type.City"))
          (`BlueprintGameplayTagLibrary.AddGameplayTag` (`self.GameplayTags`) (struct :`TagName` "Ennemi.Building.City"))
          (bind _returnvalue (`|SpawnActorFromClass` "/Game/_Main/Actors/Enemy/Buildings/BP_City.BP_City_C" (`self.GetTransform`) "Undefined" "MultiplyWithRoot" null self null null null null))
          (set `self.TileTypeVisual` _returnvalue)
          (set `self.LumberJackBuilding` _returnvalue))
        (:`NewEnumerator1`
          (`BlueprintGameplayTagLibrary.AddGameplayTag` _gameplaytags (struct :`TagName` "Tile.Type.OriginForest"))
          (`BlueprintGameplayTagLibrary.AddGameplayTag` _gameplaytags (struct :`TagName` "Tile.Type.Forest"))
          (bind _returnvalue_2 (`|SpawnActorFromClass` "/Game/_Main/Actors/Forest/ForestPart/BP_OriginForest.BP_OriginForest_C" (`self.GetTransform`) "Undefined" "MultiplyWithRoot" null null null null null))
          (set `self.TileTypeVisual` _returnvalue_2)
          (`self.Add HPs` 10))
        (:`NewEnumerator6`
          (`BlueprintGameplayTagLibrary.AddGameplayTag` _gameplaytags (struct :`TagName` "Tile.Type.Lumbercamp"))
          (bind _returnvalue_3 (`|SpawnActorFromClass` "/Game/_Main/Actors/Enemy/Buildings/BP_LumberCamp.BP_LumberCamp_C" (`self.GetTransform`) "Undefined" "MultiplyWithRoot" null self null null null null))
          (set `self.TileTypeVisual` _returnvalue_3)
          (set `self.LumberJackBuilding` _returnvalue_3)
          (`BlueprintGameplayTagLibrary.AddGameplayTag` (`self.GameplayTags`) (struct :`TagName` "Ennemi.Building.LumberCamp")))
        (:`NewEnumerator2`
          (`BlueprintGameplayTagLibrary.AddGameplayTag` _gameplaytags (struct :`TagName` "Tile.Type.Mountain"))
          (bind _returnvalue_4 (`|SpawnActorFromClass` "/Game/_Main/Actors/BP_Mountain.BP_Mountain_C" (`self.GetTransform`) "Undefined" "MultiplyWithRoot" null null null null null))
          (set `self.TileTypeVisual` _returnvalue_4)
          (`BlueprintGameplayTagLibrary.AddGameplayTag` (`self.GameplayTags`) (struct :`TagName` "Tile.Type.Mountain")))
        (:`NewEnumerator3`
          (`BlueprintGameplayTagLibrary.AddGameplayTag` _gameplaytags (struct :`TagName` "Tile.Type.Plain")))
        (:`NewEnumerator8`
          (`BlueprintGameplayTagLibrary.AddGameplayTag` _gameplaytags (struct :`TagName` "Tile.Type.PowerUp"))
          (`|SpawnActorFromClass` "/Game/_Main/Actors/BP_HumansRuins.BP_HumansRuins_C" (`self.GetTransform`) "Undefined" "MultiplyWithRoot" null null null self null)
          (`BlueprintGameplayTagLibrary.AddGameplayTag` (`self.GameplayTags`) (struct :`TagName` "Tile.Type.PowerUp")))
        (:`NewEnumerator0`
          (`BlueprintGameplayTagLibrary.AddGameplayTag` _gameplaytags (struct :`TagName` "Tile.Type.River")))
        (:`NewEnumerator4`
          (`BlueprintGameplayTagLibrary.AddGameplayTag` _gameplaytags (struct :`TagName` "Tile.Type.Village"))
          (bind _returnvalue_5 (`|SpawnActorFromClass` "/Game/_Main/Actors/Enemy/Buildings/BP_Village.BP_Village_C" (`self.GetTransform`) "Undefined" "MultiplyWithRoot" null self null null null null))
          (set `self.TileTypeVisual` _returnvalue_5)
          (set `self.LumberJackBuilding` _returnvalue_5)
          (`BlueprintGameplayTagLibrary.AddGameplayTag` (`self.GameplayTags`) (struct :`TagName` "Ennemi.Building.Village")))
        (:`NewEnumerator9`
          (`BlueprintGameplayTagLibrary.AddGameplayTag` _gameplaytags (struct :`TagName` "Ennemi.Building.Outpost"))
          (bind _returnvalue_6 (`|SpawnActorFromClass` "/Game/_Main/Actors/Enemy/Buildings/BP_OutpostSpawner.BP_OutpostSpawner_C" (`self.GetTransform`) "Undefined" "MultiplyWithRoot" null self null null null null))
          (set `self.TileTypeVisual` _returnvalue_6)
          (set `self.LumberJackBuilding` _returnvalue_6))))
    (:`then_1`
      (`KismetSystemLibrary.Delay` 0.3)
      (set `self.Coords` (`KismetMathLibrary.MakeVector2D` (`KismetMathLibrary.Conv_IntToDouble` (`KismetMathLibrary.FTrunc` _returnvalue_x)) (`KismetMathLibrary.Conv_IntToDouble` (`KismetMathLibrary.FTrunc` _returnvalue_y)))))
    (:`then_2`
      (`self.SpawnFogOfWar`)
      (`KismetSystemLibrary.Delay` 0.3)
      (`self.ChangeAdjacentTileTagToForest`))
    (:`then_3`
      (`KismetSystemLibrary.Delay` 1.0)
      (if (`BlueprintGameplayTagLibrary.HasTag` (`self.GameplayTags`) (struct :`TagName` "Ennemi.Minion.LostLumberJack") true)
        (bind _returnvalue_7 (`|SpawnActorFromClass` "/Game/_Main/Actors/Enemy/Enemy/BP_LostLumberJack.BP_LostLumberJack_C" (`self.GetTransform`) "Undefined" "MultiplyWithRoot" null self null null null))
        (set `self.EnemyMinion` _returnvalue_7)
        (elif (`BlueprintGameplayTagLibrary.HasTag` (`self.GameplayTags`) (struct :`TagName` "Ennemi.Minion.Renfort") true)
          (bind _returnvalue_8 (`|SpawnActorFromClass` "/Game/_Main/Actors/Enemy/Enemy/BP_LumberJackRenfort.BP_LumberJackRenfort_C" (`self.GetTransform`) "Undefined" "MultiplyWithRoot" null self null null null))
          (set `self.EnemyMinion` _returnvalue_8))))))

(event `UpdateTileMaterial`
  (bind _gameplaytags (`self.GameplayTags`))
  (if (not (`BlueprintGameplayTagLibrary.HasTag` (`self.GameplayTags`) (struct :`TagName` "Tile.Target")))
    (bind (_keypin _valuepin) (`|MapForEach` (`self.TileTypeMaterialID`))
      (:`then`
        (if (`BlueprintGameplayTagLibrary.HasTag` (`self.GameplayTags`) _keypin true)
          (`PrimitiveComponent.SetMaterial` (`self.Cube`) 0 _valuepin)
          (if (`BlueprintGameplayTagLibrary.HasTag` _gameplaytags (struct :`TagName` "Tile.Type.Forest") true)
            (`self.ChangeAdjacentTileTagToForest`)
            (if (and (`BlueprintGameplayTagLibrary.HasTag` _gameplaytags (struct :`TagName` "Tile.Type.Forest") true) (`BlueprintGameplayTagLibrary.HasTag` _gameplaytags (struct :`TagName` "Tile.State.AdjacentToForest") true))
              (`BlueprintGameplayTagLibrary.RemoveGameplayTag` _gameplaytags (struct :`TagName` "Tile.State.AdjacentToForest"))
              (if (and (`BlueprintGameplayTagLibrary.HasTag` _gameplaytags (struct :`TagName` "Tile.Type.Forest") true) (`BlueprintGameplayTagLibrary.HasTag` _gameplaytags (struct :`TagName` "Tile.Type.Mountain") true))
                (`BlueprintGameplayTagLibrary.RemoveGameplayTag` _gameplaytags (struct :`TagName` "Tile.Type.Forest"))))))))
    (else
      (bind (_keypin_2 _valuepin_2) (`|MapForEach` (`self.TileValidTargetMaterialID?`))
        (:`then`
          (if (`BlueprintGameplayTagLibrary.HasTag` (`self.GameplayTags`) _keypin_2 true)
            (`PrimitiveComponent.SetMaterial` (`self.Cube`) 0 _valuepin_2)))))))

(event `self.ReceiveAnyDamage`
  (params (Damage :type "Float (single-precision)") (DamageType :type "DamageType Object Reference") (InstigatedBy :type "Controller Object Reference") (DamageCauser :type "Actor Object Reference"))
  (bind _gameplaytags (`self.GameplayTags`))
  (bind (_shield _protection _deeproots _extraction _frenzy _absorption _thorn _foresthp _forestmaxhp) (break `/Game/_Main/Level/LevelDesignElement/S_TileStats` (`self.TileStats`)))
  (bind (_shield_2 _protection_2 _deeproots_2 _extraction_2 _frenzy_2 _absorption_2 _thorn_2 _foresthp_2 _forestmaxhp_2) (break `/Game/_Main/Level/LevelDesignElement/S_TileStats` (`self.TileStats`)))
  (if (> _protection 0)
    (set `self.TileStats` (make `/Game/_Main/Level/LevelDesignElement/S_TileStats` _shield (- _protection 1) _deeproots _extraction _frenzy _absorption _thorn _foresthp _forestmaxhp))
    (else
      (bind _newdamage (`self.UpdateShield` Damage))
      (bind _output_get (set `self.TileStats` (make `/Game/_Main/Level/LevelDesignElement/S_TileStats` _shield_2 _protection_2 _deeproots_2 _extraction_2 _frenzy_2 _absorption_2 _thorn_2 (`KismetMathLibrary.Clamp` (`KismetMathLibrary.FTrunc` (- _foresthp_2 _newdamage)) 0 5000) _forestmaxhp_2)))
      (if (and (== (`.ForestHP_21_6A1DECE24948764E1A3523B77914E909` (break `/Game/_Main/Level/LevelDesignElement/S_TileStats` _output_get)) 0) (`BlueprintGameplayTagLibrary.HasTag` (`self.GameplayTags`) (struct :`TagName` "Tile.Type.Forest") true))
        (`self.OnForestDestroyed`)
        (if (`BlueprintGameplayTagLibrary.HasTag` _gameplaytags (struct :`TagName` "Tile.Type.OriginForest") true)
          (`BlueprintGameplayTagLibrary.RemoveGameplayTag` _gameplaytags (struct :`TagName` "Tile.Type.OriginForest"))
          (`/Game/_Main/BP_PlayerController.GameOver` (`self.Player Controller`)))))))

(fn `Add HPs`
  (params (`+ XHp` :type Integer))
  (bind (_tilestats_shield _tilestats_protection _tilestats_deeproots _tilestats_extraction _tilestats_frenzy _tilestats_absorption _tilestats_thorn _tilestats_foresthp _tilestats_forestmaxhp) (break `/Game/_Main/Level/LevelDesignElement/S_TileStats` (`self.TileStats`)))
  (set `self.TileStats` (make `/Game/_Main/Level/LevelDesignElement/S_TileStats` _tilestats_shield _tilestats_protection _tilestats_deeproots _tilestats_extraction _tilestats_frenzy _tilestats_absorption _tilestats_thorn (+ `+ XHp` _tilestats_foresthp) (+ `+ XHp` _tilestats_forestmaxhp))))

(fn `ChangeAdjacentTileTagToForest`
  (if (`BlueprintGameplayTagLibrary.HasTag` (`self.GameplayTags`) (struct :`TagName` "Tile.Type.Forest") true)
    (for _array_element (`self.Voisins`)
      (`/Engine/EditorBlueprintResources/StandardMacros.IsValid` _array_element
        (:`Is Valid`
          (bind _gameplaytags (`/Game/_Main/Level/LevelDesignElement/BP_TileBase.GameplayTags` _array_element))
          (if (and (not (`BlueprintGameplayTagLibrary.HasTag` _gameplaytags (struct :`TagName` "Tile.State.AdjacentToForest") true)) (not (`BlueprintGameplayTagLibrary.HasTag` _gameplaytags (struct :`TagName` "Tile.Type.Forest") true)) (not (`BlueprintGameplayTagLibrary.HasTag` _gameplaytags (struct :`TagName` "Tile.Type.Mountain") true)))
            (`BlueprintGameplayTagLibrary.AddGameplayTag` _gameplaytags (struct :`TagName` "Tile.State.AdjacentToForest"))))))
    (`self.RemoveForOfWar?`)))

(fn `DestroySocket`
  ; pour destroy le socket de bush
  (`/Engine/EditorBlueprintResources/StandardMacros.IsValid` (`self.Sapling`)
    (:`Is Valid`
      (`self.K2_DestroyActor`))))

(fn `OnForestDestroyed`
  (locals (IsAdjacentToForest :type Boolean) (ISNeigbourAdjacentToForest :type Boolean) (TileToUpdate :type "/Game/_Main/Level/LevelDesignElement/BP_TileBase Object Reference"))
  (bind _gameplaytags (`self.GameplayTags`))
  (bind _saplingbuilding (`self.SaplingBuilding`))
  (bind (_sapling _turntogrowth _initiative _overviewtext _tags _canattack_ _damage _rangemin _rangemax _seeds _attacktype _saplingtype) (break `/Game/_Main/TCG/Cards/Data/S_Saplings` (`/Game/_Main/Actors/Saplings/BP_SaplingBuilding.SaplingInfos` _saplingbuilding)))
  (`|ExecutionSequence`
    (:`then_0`
      (`BlueprintGameplayTagLibrary.RemoveGameplayTag` (`self.GameplayTags`) (struct :`TagName` "Tile.Type.Forest"))
      (`self.K2_DestroyActor` (`self.TileTypeVisual`))
      (`BlueprintGameplayTagLibrary.AddGameplayTag` (`self.GameplayTags`) (struct :`TagName` "Tile.Type.Plain")))
    (:`then_1`
      (`/Engine/EditorBlueprintResources/StandardMacros.IsValid` _saplingbuilding
        (:`Is Valid`
          (`BlueprintGameplayTagLibrary.RemoveGameplayTag` (`self.GameplayTags`) _saplingtype)
          (`/Game/_Main/BP_PlayerState.AddNewCardToDiscardPile` (`/Game/_Main/BP_PlayerController.Player State` (`self.Player Controller`)) _seeds)
          (`/Game/_Main/Actors/Saplings/BP_SaplingBuilding.DestroySapling` (`self.SaplingBuilding`))
          (set `self.SaplingBuilding` null))))
    (:`then_2`
      (`BlueprintGameplayTagLibrary.RemoveGameplayTag` _gameplaytags (struct :`TagName` "Bush"))
      (`BlueprintGameplayTagLibrary.RemoveGameplayTag` _gameplaytags (struct :`TagName` "Sapling"))
      (`/Engine/EditorBlueprintResources/StandardMacros.IsValid` (`self.Sapling`)
        (:`Is Valid`
          (`/Game/_Main/BP_PlayerState.AddNewCardToDiscardPile` (`/Game/_Main/BP_PlayerController.Player State` (`self.Player Controller`)) "Bushseed")
          (`KismetSystemLibrary.PrintString` "Newcard !" true true (struct :`R` 1.0 :`G` 0.01904 :`A` 1.0))
          (`/Game/_Main/Actors/BP_TileActor.DestroyTileActorVisual` (`self.Sapling`)))))
    (:`then_3`
      (`self.UpdateTileandNeigboursAdjToForest`))
    (:`then_4`
      (`self.UpdateTileMaterial`)
      (`/Game/_Main/BP_PlayerController.Update HPs` (`self.Player Controller`) -1))))

(fn `RemoveForOfWar?`
  (locals (TileChecked :type "Float (double-precision)"))
  (bind _returnvalue (`self.K2_GetActorLocation`))
  (bind _gameplaytags (`self.GameplayTags`))
  (bind _fogofwartile (`self.FogOfWarTile`))
  (bind _playerstats_visibilityrange (break `/Game/_Main/Actors/Struct/S_PlayerStats` (`/Game/_Main/BP_PlayerController.PlayerStats` (`self.Player Controller`))))
  (if (`BlueprintGameplayTagLibrary.HasTag` (`self.GameplayTags`) (struct :`TagName` "Tile.Type.Forest") true)
    (`|ExecutionSequence`
      (:`then_0`
        (bind _outhits (`KismetSystemLibrary.SphereTraceMultiForObjects` _returnvalue _returnvalue (`KismetMathLibrary.Conv_IntToDouble` (- (* _playerstats_visibilityrange 100) 40)) (`|MakeArray` "ObjectTypeQuery7" :!type "EObjectTypeQuery Enum")))
        (for _array_element _outhits
          (bind _asbp_tile_base (cast `/Game/_Main/Level/LevelDesignElement/BP_TileBase` (`.HitActor` (`GameplayStatics.BreakHitResult` _array_element))))
          (bind _gameplaytags_2 (`/Game/_Main/Level/LevelDesignElement/BP_TileBase.GameplayTags` _asbp_tile_base))
          (`BlueprintGameplayTagLibrary.RemoveGameplayTag` _gameplaytags_2 (struct :`TagName` "Tile.State.Fogged"))
          (`BlueprintGameplayTagLibrary.AddGameplayTag` _gameplaytags_2 (struct :`TagName` "Tile.State.Revealed"))
          (bind _fogofwartile_2 (`/Game/_Main/Level/LevelDesignElement/BP_TileBase.FogOfWarTile` _asbp_tile_base))
          (`/Engine/EditorBlueprintResources/StandardMacros.IsValid` _fogofwartile_2
            (:`Is Valid`
              (`self.K2_DestroyActor` _fogofwartile_2)
              (bind _enemyminion (`/Game/_Main/Level/LevelDesignElement/BP_TileBase.EnemyMinion` _asbp_tile_base))
              (`/Engine/EditorBlueprintResources/StandardMacros.IsValid` _enemyminion
                (:`Is Valid`
                  (`/Game/_Main/Actors/Enemy/BP_LumberJackBase.Visible?` _enemyminion)))))))
      (:`then_1`
        (`BlueprintGameplayTagLibrary.RemoveGameplayTag` _gameplaytags (struct :`TagName` "Tile.State.Fogged"))
        (`BlueprintGameplayTagLibrary.AddGameplayTag` _gameplaytags (struct :`TagName` "Tile.State.Revealed"))
        (`/Engine/EditorBlueprintResources/StandardMacros.IsValid` _fogofwartile
          (:`Is Valid`
            (`self.K2_DestroyActor` _fogofwartile)))))))

(fn `SetupNeigbours`
  (params (TileCoords :type "Map of Vector2D Structure to /Game/_Main/Level/LevelDesignElement/BP_TileBase Object Reference"))
  (bind _coords (`self.Coords`))
  (bind _voisins (`self.Voisins`))
  (bind _value (`BlueprintMapLibrary.Map_Find` TileCoords (+ _coords (0.0 100.0))))
  (bind _value_2 (`BlueprintMapLibrary.Map_Find` TileCoords (+ _coords (-100.0 0.0))))
  (bind _value_3 (`BlueprintMapLibrary.Map_Find` TileCoords (+ _coords (0.0 -100.0))))
  (bind _value_4 (`BlueprintMapLibrary.Map_Find` TileCoords (+ _coords (100.0 0.0))))
  (`|ExecutionSequence`
    (:`then_0`
      (`/Engine/EditorBlueprintResources/StandardMacros.IsValid` _value_4
        (:`Is Valid`
          (`KismetArrayLibrary.Array_Add` _voisins _value_4))))
    (:`then_1`
      (`/Engine/EditorBlueprintResources/StandardMacros.IsValid` _value
        (:`Is Valid`
          (`KismetArrayLibrary.Array_Add` _voisins _value))))
    (:`then_2`
      (`/Engine/EditorBlueprintResources/StandardMacros.IsValid` _value_2
        (:`Is Valid`
          (`KismetArrayLibrary.Array_Add` _voisins _value_2))))
    (:`then_3`
      (`/Engine/EditorBlueprintResources/StandardMacros.IsValid` _value_3
        (:`Is Valid`
          (`KismetArrayLibrary.Array_Add` _voisins _value_3))))))

(fn `SpawnFogOfWar`
  (if (not (`BlueprintGameplayTagLibrary.HasTag` (`self.GameplayTags`) (struct :`TagName` "Tile.Type.Mountain") true))
    (bind _returnvalue (`|SpawnActorFromClass` "/Game/_Main/Level/LevelDesignElement/BP_FogOfWarTile.BP_FogOfWarTile_C" (`self.GetTransform`) "Undefined" "MultiplyWithRoot" null null))
    (set `self.FogOfWarTile` _returnvalue)
    (`BlueprintGameplayTagLibrary.AddGameplayTag` (`self.GameplayTags`) (struct :`TagName` "Tile.State.Fogged"))))

(fn `Update SaplingType`
  (`BlueprintGameplayTagLibrary.AddGameplayTag` (`self.GameplayTags`) (`.SaplingType_70_0C358B7A462984C81B2A1D92076E3AFD` (break `/Game/_Main/TCG/Cards/Data/S_Saplings` (`/Game/_Main/Actors/Saplings/BP_SaplingBuilding.SaplingInfos` (`self.SaplingBuilding`))))))

(fn `UpdateAdjacentToForest`
  (locals (IsAdjacentToForest :type Boolean))
  (bind _gameplaytags (`self.GameplayTags`))
  (for _array_element (`self.Voisins`)
    (`/Engine/EditorBlueprintResources/StandardMacros.IsValid` _array_element
      (:`Is Valid`
        (bind _gameplaytags_2 (`/Game/_Main/Level/LevelDesignElement/BP_TileBase.GameplayTags` _array_element))
        (bind _returnvalue (`BlueprintGameplayTagLibrary.HasTag` _gameplaytags_2 (struct :`TagName` "Tile.Type.Forest") true))
        (if (and (`BlueprintGameplayTagLibrary.HasTag` _gameplaytags_2 (struct :`TagName` "Tile.State.AdjacentToForest") true) (not _returnvalue) (not (`local.IsAdjacentToForest`)))
          (set `local.IsAdjacentToForest` false)
          (elif _returnvalue
            (set `local.IsAdjacentToForest` true))))))
  (`|ExecutionSequence`
    (:`then_0`
      (if (not (`local.IsAdjacentToForest`))
        (`BlueprintGameplayTagLibrary.RemoveGameplayTag` _gameplaytags (struct :`TagName` "Tile.State.AdjacentToForest"))
        (else
          (`BlueprintGameplayTagLibrary.AddGameplayTag` _gameplaytags (struct :`TagName` "Tile.State.AdjacentToForest")))))))

(fn `UpdateShield`
  (params (Damage :type "Float (double-precision)"))
  (returns (NewDamage :type "Float (double-precision)"))
  (bind (_shield _protection _deeproots _extraction _frenzy _absorption _thorn _foresthp _forestmaxhp) (break `/Game/_Main/Level/LevelDesignElement/S_TileStats` (`self.TileStats`)))
  (if (> _shield 0)
    (set `self.TileStats` (make `/Game/_Main/Level/LevelDesignElement/S_TileStats` (`KismetMathLibrary.Clamp` (`KismetMathLibrary.FTrunc` (- _shield Damage)) 0 5000) _protection _deeproots _extraction _frenzy _absorption _thorn _foresthp _forestmaxhp))
    (if (== _shield 0)
      (`self.K2_DestroyActor` (`self.ShieldSlot`))
      (set `self.ShieldSlot` null))
    (return (`KismetMathLibrary.FClamp` (- (`local.Damage`) _shield) 0.0 5000.0))
    (else
      (return (`local.Damage`)))))

(fn `UpdateTileandNeigboursAdjToForest`
  (`self.UpdateAdjacentToForest`)
  (for _array_element (`self.Voisins`)
    (`/Engine/EditorBlueprintResources/StandardMacros.IsValid` _array_element
      (:`Is Valid`
        (`self.UpdateAdjacentToForest` _array_element)))))

(fn `UserConstructionScript`
  (bind (_returnvalue_x _returnvalue_y) (`KismetMathLibrary.BreakVector` (`self.K2_GetActorLocation`)))
  (set `self.Coords` (`KismetMathLibrary.MakeVector2D` (`KismetMathLibrary.Conv_IntToDouble` (`KismetMathLibrary.FTrunc` _returnvalue_x)) (`KismetMathLibrary.Conv_IntToDouble` (`KismetMathLibrary.FTrunc` _returnvalue_y)))))