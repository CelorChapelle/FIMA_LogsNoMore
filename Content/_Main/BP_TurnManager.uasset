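; Turn manager actor that resolves player-side actions, then enemy actions, when EndTurn fires.
; Each phase gathers interface implementers (BPI_EndPlayerTurn, then BPI_EnemiTurn) and selection-sorts them by priority, lowest first.
; Recursive events execute each actor in sequence, delaying by its reported duration.
; PlayingTurn blocks re-entry while the HUD is hit-test invisible; both reset only after the last enemy acts, so never with zero enemies.
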(event `self.ReceiveBeginPlay`
  (bind _asbp_player_controller (cast `/Game/_Main/BP_PlayerController` (`GameplayStatics.GetPlayerController` 0)))
  (set `self.Player Controller` _asbp_player_controller))

(event `EndTurn`
  (bind _turn_list (`self.Turn List`))
  (bind _turn_list_2 (`self.Turn List`))
  (bind _maxindex (`self.MaxIndex`))
  (bind (_output_priority _output_actor) (break `/Game/_Main/Actors/Struct/S_PrioritySort` (`|GetArrayItem` _turn_list _maxindex)))
  (if (not (`self.PlayingTurn`))
    (set `self.PlayingTurn` true)
    (`Widget.SetVisibility` (`/Game/_Main/BP_PlayerController.HUD` (`self.Player Controller`)) "HitTestInvisible")
    (bind _outactors (`GameplayStatics.GetAllActorsWithInterface` "/Game/_Main/BPI_EndPlayerTurn.BPI_EndPlayerTurn_C"))
    (for _array_element _outactors
      (bind _priority (message `/Game/_Main/BPI_EndPlayerTurn.GetPlayerTurnPriority` _array_element))
      (`KismetArrayLibrary.Array_Add` (`self.Turn List`) (make `/Game/_Main/Actors/Struct/S_PrioritySort` _priority _array_element)))
    (`KismetArrayLibrary.Array_Clear` (`self.SortedList`))
    (while (`KismetArrayLibrary.Array_IsNotEmpty` (`self.Turn List`))
      (set `self.MaxIndex` 0)
      (for _index (range 1 (`KismetArrayLibrary.Array_Length` (`self.Turn List`)))
        (if (< (`.Priority_4_946F9FBF472F6C18DE59C98D81D2E0EE` (break `/Game/_Main/Actors/Struct/S_PrioritySort` (`|GetArrayItem` _turn_list_2 _index))) (`.Priority_4_946F9FBF472F6C18DE59C98D81D2E0EE` (break `/Game/_Main/Actors/Struct/S_PrioritySort` (`|GetArrayItem` _turn_list_2 (`self.MaxIndex`)))))
          (set `self.MaxIndex` _index)))
      (`KismetArrayLibrary.Array_Add` (`self.SortedList`) _output_actor)
      (`KismetArrayLibrary.Array_Remove` _turn_list _maxindex))
    (set `self.CurrentIndex` 0)
    (`self.ExecuteAllPlayerTurn`)))

(event `ExecuteAllPlayerTurn`
  (bind _sortedlist (`self.SortedList`))
  (bind _output (`|GetArrayItem` _sortedlist (`self.CurrentIndex`)))
  (if (< (`self.CurrentIndex`) (`KismetArrayLibrary.Array_Length` _sortedlist))
    (bind (_priority _turntime) (message `/Game/_Main/BPI_EndPlayerTurn.GetPlayerTurnPriority` _output))
    (message `/Game/_Main/BPI_EndPlayerTurn.Execute Player Turn` _output)
    (`KismetSystemLibrary.Delay` _turntime)
    (set `self.CurrentIndex` (+ (`self.CurrentIndex`) 1))
    (`self.ExecuteAllPlayerTurn`)
    (else
      (`self.PlayAllEnemyTurn`))))

(event `PlayAllEnemyTurn`
  (bind _turn_list (`self.Turn List`))
  (bind _maxindex (`self.MaxIndex`))
  (bind _turn_list_2 (`self.Turn List`))
  (bind (_output_priority _output_actor) (break `/Game/_Main/Actors/Struct/S_PrioritySort` (`|GetArrayItem` _turn_list _maxindex)))
  (`KismetArrayLibrary.Array_Clear` (`self.Turn List`))
  (bind _outactors (`GameplayStatics.GetAllActorsWithInterface` "/Game/_Main/BPI_EnemiTurn.BPI_EnemiTurn_C"))
  (for _array_element _outactors
    (bind _priority (message `/Game/_Main/BPI_EnemiTurn.GetEnemiTurnPriority` _array_element))
    (`KismetArrayLibrary.Array_Add` (`self.Turn List`) (make `/Game/_Main/Actors/Struct/S_PrioritySort` _priority _array_element)))
  (`KismetArrayLibrary.Array_Clear` (`self.SortedList`))
  (while (`KismetArrayLibrary.Array_IsNotEmpty` (`self.Turn List`))
    (set `self.MaxIndex` 0)
    (for _index (range 1 (`KismetArrayLibrary.Array_Length` (`self.Turn List`)))
      (if (< (`.Priority_4_946F9FBF472F6C18DE59C98D81D2E0EE` (break `/Game/_Main/Actors/Struct/S_PrioritySort` (`|GetArrayItem` _turn_list_2 _index))) (`.Priority_4_946F9FBF472F6C18DE59C98D81D2E0EE` (break `/Game/_Main/Actors/Struct/S_PrioritySort` (`|GetArrayItem` _turn_list_2 (`self.MaxIndex`)))))
        (set `self.MaxIndex` _index)))
    (`KismetArrayLibrary.Array_Add` (`self.SortedList`) _output_actor)
    (`KismetArrayLibrary.Array_Remove` _turn_list _maxindex))
  (set `self.CurrentIndex` 0)
  (`self.ExcecuteAllEnemyTurn`))

(event `ExcecuteAllEnemyTurn`
  (bind _sortedlist (`self.SortedList`))
  (bind _output (`|GetArrayItem` _sortedlist (`self.CurrentIndex`)))
  (if (< (`self.CurrentIndex`) (`KismetArrayLibrary.Array_Length` _sortedlist))
    (bind (_priority _actionduration) (message `/Game/_Main/BPI_EnemiTurn.GetEnemiTurnPriority` _output))
    (message `/Game/_Main/BPI_EnemiTurn.Execute Enemi Turn` _output)
    (`KismetSystemLibrary.Delay` _actionduration)
    (set `self.CurrentIndex` (+ (`self.CurrentIndex`) 1))
    (if (!= (`KismetArrayLibrary.Array_Length` (`self.SortedList`)) (`self.CurrentIndex`))
      (`self.ExcecuteAllEnemyTurn`)
      (else
        (set `self.PlayingTurn` false)
        (`Widget.SetVisibility` (`/Game/_Main/BP_PlayerController.HUD` (`self.Player Controller`)) "Visible")))))

(fn `UserConstructionScript`)