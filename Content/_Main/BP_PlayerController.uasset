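; Player controller for a turn-based card game on a tile map, handling card targeting, sapling moves, mana and end of turn.
; BeginPlay creates the HUD and the map, card effect and turn managers, then draws the first hand after a delay workaround.
; Tick traces under the cursor, flagging tile validity through gameplay tags and materials.
; Left click plays the card or relocates a sapling; right click cancels a card.
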(event `self.ReceiveBeginPlay`
  (bind _returnvalue (subsystem `EnhancedInputLocalPlayerSubsystem`))
  (bind (_playerstats_visibilityrange _playerstats_mana _playerstats_manaperturn _playerstats_tempovermana _playerstats_drawcardperturn) (break `/Game/_Main/Actors/Struct/S_PlayerStats` (`self.PlayerStats`)))
  ;[0.05098 0.05098 0.05098] Add Mapping Context
  (`/Engine/EditorBlueprintResources/StandardMacros.IsValid` _returnvalue
    (:`Is Valid`
      (`EnhancedInputSubsystemInterface.AddMappingContext` _returnvalue "/Game/_Main/Input/IMC_Nomorelogs.IMC_Nomorelogs" 0 (struct))
      (bind _asbp_player_state (cast `/Game/_Main/BP_PlayerState` (`GameplayStatics.GetPlayerState` 0)))
      (set `self.Player State` _asbp_player_state)
      (bind _returnvalue_2 (`|CreateWidget` "/Game/_Main/TCG/Cards/Widget/WBP_HUD.WBP_HUD_C"))
      (set `self.HUD` _returnvalue_2)
      (`UserWidget.AddToViewport` _returnvalue_2 0)
      (set `self.bShowMouseCursor` true)
      (bind _returnvalue_3 (`|SpawnActorFromClass` "/Game/_Main/BP_MapManager.BP_MapManager_C" (`KismetMathLibrary.MakeTransform` (0.0 0.0 0.0)) "Undefined" "MultiplyWithRoot" null null))
      (set `self.Map Manager` _returnvalue_3)
      (bind _returnvalue_4 (`|SpawnActorFromClass` "/Game/_Main/BP_CardEffectManager.BP_CardEffectManager_C" (`KismetMathLibrary.MakeTransform` (0.0 0.0 0.0)) "Undefined" "MultiplyWithRoot" null null))
      (set `self.CardEffectManager` _returnvalue_4)
      (bind _returnvalue_5 (`|SpawnActorFromClass` "/Game/_Main/BP_TurnManager.BP_TurnManager_C" (`KismetMathLibrary.MakeTransform` (0.0 0.0 0.0)) "Undefined" "MultiplyWithRoot" null null))
      (set `self.TurnManager` _returnvalue_5)
      (`self.UpdatePlayersStats`)
      (bind _asbp_camera_character (cast `/Game/_Main/BP_CameraCharacter` (`GameplayStatics.GetPlayerPawn` 0)))
      (set `self.Camera Character` _asbp_camera_character)
      ; Soucis au lancement du jeu (pansement)
      (`KismetSystemLibrary.Delay` 1.0)
      (`/Game/_Main/BP_PlayerState.DrawCard` (`self.Player State`) _playerstats_drawcardperturn))))

(event `self.ReceiveTick`
  (params (DeltaSeconds :type "Float (single-precision)"))
  (`self.CheckTileWhileDragOn`))

(event `Key|LeftMouseButton`
  (params (Key :type "Key Structure"))
  (bind _undercursortile (`self.UnderCursorTile`))
  (bind _potentialtargets (`self.PotentialTargets`))
  (bind _currenttileselected (`self.CurrentTileSelected`))
  (bind _currenttileselected_2 (`self.CurrentTileSelected`))
  (bind _player_state (`self.Player State`))
  (bind _gameplaytags (`/Game/_Main/Level/LevelDesignElement/BP_TileBase.GameplayTags` (`self.UnderCursorTile`)))
  (bind _saplingbuilding (`/Game/_Main/Level/LevelDesignElement/BP_TileBase.SaplingBuilding` _currenttileselected_2))
  (:`Pressed`
    (`/Engine/EditorBlueprintResources/StandardMacros.IsValid` (`self.TargetingActor`)
      (:`Is Valid`
        (`/Engine/EditorBlueprintResources/StandardMacros.IsValid` (`self.UnderCursorTile`)
          (:`Is Valid`
            ; Est-ce qu'on a une cible valide ?
            (if (`BlueprintGameplayTagLibrary.HasTag` _gameplaytags (struct :`TagName` "Tile.Target.IsValid") true)
              (`BlueprintGameplayTagLibrary.RemoveGameplayTag` _gameplaytags (struct :`TagName` "Tile.Target.IsValid"))
              (`/Game/_Main/Level/LevelDesignElement/BP_TileBase.UpdateMaterial` (`self.UnderCursorTile`))
              (`KismetSystemLibrary.PrintString` (`BlueprintGameplayTagLibrary.GetDebugStringFromGameplayTagContainer` _gameplaytags) true true (struct :`R` 1.0 :`B` 0.946164 :`A` 1.0))
              (`self.K2_DestroyActor` (`self.TargetingActor`))
              (set `self.bShowMouseCursor` true)
              (if (== (`self.PlayingCardEffect`) 0)
                (`/Game/_Main/BP_PlayerState.PlayCard` _player_state (`self.PlayingCardInstance`) (`self.UnderCursorTile`))
                (if (`/Game/_Main/BP_PlayerState.Replicate?` _player_state)
                  (`self.UnplayCurrentCard`)
                  (`Widget.RemoveFromParent` (`/Game/_Main/TCG/Cards/Widget/WBP_HUD.CurrentVisibleCard` (`self.HUD`)))
                  (set `/Game/_Main/BP_PlayerState.Replicate?` false (`self.Player State`))
                  (else
                    (`Widget.RemoveFromParent` (`/Game/_Main/TCG/Cards/Widget/WBP_HUD.CurrentVisibleCard` (`self.HUD`)))))
                (`self.ClearCardInstance` (struct))
                (else
                  ; On Moove
                  (`self.K2_SetActorLocation` _saplingbuilding (`self.K2_GetActorLocation` (`self.UnderCursorTile`)) false false)
                  (`BlueprintGameplayTagLibrary.RemoveGameplayTag` (`/Game/_Main/Level/LevelDesignElement/BP_TileBase.GameplayTags` _currenttileselected) (`.SaplingType_70_0C358B7A462984C81B2A1D92076E3AFD` (break `/Game/_Main/TCG/Cards/Data/S_Saplings` (`/Game/_Main/Actors/Saplings/BP_SaplingBuilding.SaplingInfos` (`/Game/_Main/Level/LevelDesignElement/BP_TileBase.SaplingBuilding` _currenttileselected)))))
                  (bind _output_get (set `/Game/_Main/Level/LevelDesignElement/BP_TileBase.SaplingBuilding` _saplingbuilding _undercursortile))
                  (set `/Game/_Main/Actors/Saplings/BP_SaplingBuilding.LinkedTile_0` _undercursortile _output_get)
                  (set `/Game/_Main/Level/LevelDesignElement/BP_TileBase.SaplingBuilding` null _currenttileselected_2)
                  (`BlueprintGameplayTagLibrary.AddGameplayTag` (`/Game/_Main/Level/LevelDesignElement/BP_TileBase.GameplayTags` _undercursortile) (`.SaplingType_70_0C358B7A462984C81B2A1D92076E3AFD` (break `/Game/_Main/TCG/Cards/Data/S_Saplings` (`/Game/_Main/Actors/Saplings/BP_SaplingBuilding.SaplingInfos` (`/Game/_Main/Level/LevelDesignElement/BP_TileBase.SaplingBuilding` _undercursortile)))))
                  (set `self.bShowMouseCursor` true)
                  (set `self.PlayingCardEffect` 0)
                  (set `self.MooveEffect` "NewEnumerator0")
                  (for _array_element _potentialtargets
                    (`BlueprintGameplayTagLibrary.RemoveGameplayTag` (`/Game/_Main/Level/LevelDesignElement/BP_TileBase.GameplayTags` _array_element) (struct :`TagName` "Tile.Target.IsValid")))
                  (`KismetArrayLibrary.Array_Clear` _potentialtargets))))))))))

(event `Key|RightMouseButton`
  (params (Key :type "Key Structure"))
  (:`Pressed`
    (if (== (`self.PlayingCardEffect`) 0)
      (`self.UnplayCurrentCard`))))

(event `Key|F`
  (params (Key :type "Key Structure"))
  (:`Pressed`
    (`/Game/_Main/BP_PlayerState.UpdateRewardCard` (`self.Player State`))))

(event `UnplayCurrentCard`
  (bind _targetingactor (`self.TargetingActor`))
  (bind _currentvisiblecard (`/Game/_Main/TCG/Cards/Widget/WBP_HUD.CurrentVisibleCard` (`self.HUD`)))
  (set `self.bShowMouseCursor` true)
  (`/Engine/EditorBlueprintResources/StandardMacros.IsValid` _currentvisiblecard
    (:`Is Valid`
      (`/Game/_Main/TCG/Cards/Widget/WBP_HUD.AddNewCard` (`self.HUD`) (`self.PlayingCardInstance`))
      (`Widget.RemoveFromParent` _currentvisiblecard))
    (:`Is Not Valid`
      _))
  (`/Engine/EditorBlueprintResources/StandardMacros.IsValid` _targetingactor
    (:`Is Valid`
      (`self.K2_DestroyActor` _targetingactor))))

(event `EndTurn`
  (bind (_playerstats_visibilityrange _playerstats_mana _playerstats_manaperturn _playerstats_tempovermana _playerstats_drawcardperturn) (break `/Game/_Main/Actors/Struct/S_PlayerStats` (`self.PlayerStats`)))
  (bind _hud (`self.HUD`))
  (set `self.bShowMouseCursor` false)
  ; PlayAllEffect&Enemi
  (`/Game/_Main/BP_TurnManager.EndTurn` (`self.TurnManager`))
  (`self.UpdatePlayersStats`)
  (set `self.bShowMouseCursor` true)
  (`/Game/_Main/BP_PlayerState.DiscardFullHand` (`self.Player State`))
  (`/Game/_Main/TCG/Cards/Widget/WBP_HUD.ClearHand` _hud)
  (`/Game/_Main/BP_PlayerState.DrawCard` (`self.Player State`) _playerstats_drawcardperturn)
  (`/Game/_Main/TCG/Cards/Widget/WBP_ButtonOriginForestPower.RefreshButton` (`/Game/_Main/TCG/Cards/Widget/WBP_HUD.WBP_BuyBushSeed` _hud)))

(fn `CheckTileWhileDragOn`
  (locals (TempCardGameplayTag :type "GameplayTagContainer Structure"))
  (bind (_hitresult _returnvalue) (`self.GetHitResultUnderCursorByChannel` "TraceTypeQuery1"))
  (bind (_hitresult_2 _returnvalue_2) (`self.GetHitResultUnderCursorByChannel` "TraceTypeQuery1"))
  (bind _undercursortile (`self.UnderCursorTile`))
  (bind _undercursortile_2 (`self.UnderCursorTile`))
  (bind _undercursortile_3 (`self.UnderCursorTile`))
  (bind _undercursortile_4 (`self.UnderCursorTile`))
  (bind (_bblockinghit _binitialoverlap _time _distance _location _impactpoint _normal _impactnormal _physmat _hitactor) (`GameplayStatics.BreakHitResult` _hitresult))
  (bind (_bblockinghit_2 _binitialoverlap_2 _time_2 _distance_2 _location_2 _impactpoint_2 _normal_2 _impactnormal_2 _physmat_2 _hitactor_2) (`GameplayStatics.BreakHitResult` _hitresult_2))
  (bind _gameplaytags (`/Game/_Main/Level/LevelDesignElement/BP_TileBase.GameplayTags` (`self.UnderCursorTile`)))
  (bind _gameplaytags_2 (`/Game/_Main/Level/LevelDesignElement/BP_TileBase.GameplayTags` _undercursortile))
  (bind _gameplaytags_3 (`/Game/_Main/Level/LevelDesignElement/BP_TileBase.GameplayTags` (`self.UnderCursorTile`)))
  (bind _cube (`/Game/_Main/Level/LevelDesignElement/BP_TileBase.Cube` _undercursortile_4))
  (bind _gameplaytags_4 (`/Game/_Main/Level/LevelDesignElement/BP_TileBase.GameplayTags` _undercursortile_3))
  (bind (_type _cost _instigatortag _tags _exhaust_ _text _target _mandatorytarget) (break `/Game/_Main/TCG/Cards/Data/S_CardData` (`.CardData_18_E97FEC6A494667101BBA969E8A2DCF93` (break `/Game/_Main/TCG/Cards/Data/S_CardInstance` (`self.PlayingCardInstance`)))))
  (switch `/Game/_Main/TCG/Cards/Data/E_SaplingsMoveEffect` (`self.MooveEffect`)
    (:`NewEnumerator0`
      (if _returnvalue
        (bind _asbp_tile_base (cast `/Game/_Main/Level/LevelDesignElement/BP_TileBase` _hitactor))
        (`self.Print Tile Stats` _asbp_tile_base)
        (if (!= (`self.UnderCursorTile`) _hitactor)
          (`/Engine/EditorBlueprintResources/StandardMacros.IsValid` (`self.TargetingActor`)
            (:`Is Valid`
              (`/Engine/EditorBlueprintResources/StandardMacros.IsValid` _undercursortile_2
                (:`Is Valid`
                  (`BlueprintGameplayTagLibrary.RemoveGameplayTag` _gameplaytags_3 (struct :`TagName` "Tile.Target.IsNotValid"))
                  (`BlueprintGameplayTagLibrary.RemoveGameplayTag` _gameplaytags_3 (struct :`TagName` "Tile.Target.IsValid"))
                  (`/Game/_Main/Level/LevelDesignElement/BP_TileBase.UpdateMaterial` _undercursortile_2))
                (:`Is Not Valid`
                  _))
              (set `self.UnderCursorTile` _asbp_tile_base)
              (if (or (`BlueprintGameplayTagLibrary.HasTag` _gameplaytags (struct :`TagName` "Ennemi.Building")) (`BlueprintGameplayTagLibrary.HasTag` _gameplaytags (struct :`TagName` "Ennemi.Minion")))
                (`BlueprintGameplayTagLibrary.AddGameplayTag` _gameplaytags_2 (struct :`TagName` "Tile.Target.IsNotValid") :!label _label)
                (elif (and (`BlueprintGameplayTagLibrary.HasAnyTags` (`/Game/_Main/Level/LevelDesignElement/BP_TileBase.GameplayTags` (`self.UnderCursorTile`)) _mandatorytarget true) (`BlueprintGameplayTagLibrary.HasAnyTags` (`/Game/_Main/Level/LevelDesignElement/BP_TileBase.GameplayTags` (`self.UnderCursorTile`)) _target true))
                  (`BlueprintGameplayTagLibrary.AddGameplayTag` _gameplaytags_2 (struct :`TagName` "Tile.Target.IsValid"))
                  (else
                    (goto _label))))
              (`/Game/_Main/Level/LevelDesignElement/BP_TileBase.UpdateMaterial` _undercursortile))))
        (else
          (`/Engine/EditorBlueprintResources/StandardMacros.IsValid` (`self.TargetingActor`)
            (:`Is Valid`
              (`/Engine/EditorBlueprintResources/StandardMacros.IsValid` _undercursortile_3
                (:`Is Valid`
                  (`BlueprintGameplayTagLibrary.RemoveGameplayTag` _gameplaytags_4 (struct :`TagName` "Tile.Target.IsNotValid"))
                  (`BlueprintGameplayTagLibrary.RemoveGameplayTag` _gameplaytags_4 (struct :`TagName` "Tile.Target.IsValid"))
                  (`/Game/_Main/Level/LevelDesignElement/BP_TileBase.UpdateMaterial` (`self.UnderCursorTile`))
                  (set `self.UnderCursorTile` null))))))))
    (:`NewEnumerator13`
      (if _returnvalue_2 :!label _label_2
        (bind _asbp_tile_base_2 (cast `/Game/_Main/Level/LevelDesignElement/BP_TileBase` _hitactor_2))
        (if (!= (`self.UnderCursorTile`) _hitactor_2)
          (`/Engine/EditorBlueprintResources/StandardMacros.IsValid` (`self.TargetingActor`)
            (:`Is Valid`
              (`/Engine/EditorBlueprintResources/StandardMacros.IsValid` (`self.UnderCursorTile`)
                (:`Is Valid`
                  (if (`BlueprintGameplayTagLibrary.HasTag` (`/Game/_Main/Level/LevelDesignElement/BP_TileBase.GameplayTags` _undercursortile_4) (struct :`TagName` "Tile.Target.IsValid") true)
                    (`PrimitiveComponent.SetMaterial` _cube 0 "/Game/_Main/Materials/MI_BaseColor_DarkGreen.MI_BaseColor_DarkGreen")
                    (else
                      (`/Game/_Main/Level/LevelDesignElement/BP_TileBase.UpdateMaterial` _undercursortile_4))))
                (:`Is Not Valid`
                  _))
              (set `self.UnderCursorTile` _asbp_tile_base_2)
              (if (`BlueprintGameplayTagLibrary.HasTag` (`/Game/_Main/Level/LevelDesignElement/BP_TileBase.GameplayTags` (`self.UnderCursorTile`)) (struct :`TagName` "Tile.Target.IsValid") true)
                (`PrimitiveComponent.SetMaterial` _cube 0 "/Game/_Main/Materials/MI_BaseColor_Target.MI_BaseColor_Target")
                (else
                  (`PrimitiveComponent.SetMaterial` _cube 0 "/Game/_Main/Materials/MI_BaseColor_Red.MI_BaseColor_Red"))))))
        (else
          (`/Engine/EditorBlueprintResources/StandardMacros.IsValid` (`self.TargetingActor`)
            (:`Is Valid`
              (`/Engine/EditorBlueprintResources/StandardMacros.IsValid` (`self.UnderCursorTile`)
                (:`Is Valid`
                  (if (`BlueprintGameplayTagLibrary.HasTag` (`/Game/_Main/Level/LevelDesignElement/BP_TileBase.GameplayTags` (`self.UnderCursorTile`)) (struct :`TagName` "Tile.Target.IsValid") true)
                    (`PrimitiveComponent.SetMaterial` (`/Game/_Main/Level/LevelDesignElement/BP_TileBase.Cube` (`self.UnderCursorTile`)) 0 "/Game/_Main/Materials/MI_BaseColor_DarkGreen.MI_BaseColor_DarkGreen")
                    (set `self.UnderCursorTile` null)))))))))
    (:`NewEnumerator14`
      (goto _label_2))))

(fn `ClearCardInstance`
  (params (CardInstance :type "/Game/_Main/TCG/Cards/Data/S_CardInstance Structure"))
  (set `self.PlayingCardInstance` CardInstance))

(fn `FindTargetInRadiusOfATile`
  (params (CurrentTarget :type "/Game/_Main/Level/LevelDesignElement/BP_TileBase Object Reference") (Radius :type "Float (double-precision)"))
  (returns (TileInRange :type "Array of /Game/_Main/Level/LevelDesignElement/BP_TileBase Object Reference"))
  (bind _returnvalue (`self.K2_GetActorLocation` CurrentTarget))
  (`|ExecutionSequence`
    (:`then_0`
      (bind _outhits (`KismetSystemLibrary.SphereTraceMultiForObjects` :`Start` _returnvalue :`End` _returnvalue :`Radius` Radius :`ObjectTypes` (`|MakeArray` "ObjectTypeQuery7" :!type "EObjectTypeQuery Enum") :`DrawDebugType` "ForDuration"))
      (for _array_element _outhits
        (bind _asbp_tile_base (cast `/Game/_Main/Level/LevelDesignElement/BP_TileBase` (`.HitActor` (`GameplayStatics.BreakHitResult` _array_element))))
        (if (`BlueprintGameplayTagLibrary.HasTag` (`/Game/_Main/Level/LevelDesignElement/BP_TileBase.GameplayTags` _asbp_tile_base) (struct :`TagName` "Tile.Type.Forest"))
          (`KismetArrayLibrary.Array_Add` (`self.PotentialTargets`) _asbp_tile_base))))
    (:`then_1`
      (return (`self.PotentialTargets`)))))

(fn `GameOver`
  (`KismetSystemLibrary.PrintString` "GAME OVER" true true (struct :`R` 1.0 :`B` 0.000954 :`A` 1.0) 200.0 "Gameover"))

(fn `Get a Reward`
  (`KismetSystemLibrary.PrintString` "REWARD" true true (struct :`R` 0.166477 :`G` 1.0 :`B` 0.001207 :`A` 1.0) 2.0 "REWARD"))

(fn `Print Tile Stats`
  (params (Target :type "/Game/_Main/Level/LevelDesignElement/BP_TileBase Object Reference"))
  (locals (NewLocalVar :type "/Game/_Main/Level/LevelDesignElement/BP_TileBase Object Reference"))
  (bind _output_get (set `local.NewLocalVar` Target))
  (`|ExecutionSequence`
    (:`then_0`
      (bind (_shield _protection _deeproots _extraction _frenzy _absorption _thorn _foresthp) (break `/Game/_Main/Level/LevelDesignElement/S_TileStats` (`/Game/_Main/Level/LevelDesignElement/BP_TileBase.TileStats` _output_get)))
      (if (> _foresthp 0)
        (`KismetSystemLibrary.PrintString` (`KismetStringLibrary.Concat_StrStr` "HP : " (`KismetStringLibrary.Conv_IntToString` _foresthp)) true true (struct :`R` 1.0 :`G` 0.019515 :`A` 1.0) 0.1 "HPs")))
    (:`then_1`
      (if (> _shield 0)
        (`KismetSystemLibrary.PrintString` (`KismetStringLibrary.Concat_StrStr` "Bark : " (`KismetStringLibrary.Conv_IntToString` _shield)) true true (struct :`R` 0.298222 :`G` 0.010364 :`B` 1.0 :`A` 1.0) 0.1 "Shield")))
    (:`then_2`
      (`KismetSystemLibrary.PrintString` (`BlueprintGameplayTagLibrary.GetDebugStringFromGameplayTagContainer` (`/Game/_Main/Level/LevelDesignElement/BP_TileBase.GameplayTags` _output_get)) true true (struct :`R` 1.0 :`G` 0.821071 :`A` 1.0) 0.1 "TAGS"))))

(fn `SpawnTargettingActor`
  (`/Engine/EditorBlueprintResources/StandardMacros.IsValid` (`self.TargetingActor`)
    (:`Is Not Valid`
      (bind _returnvalue (`|SpawnActorFromClass` "/Game/_Main/Actors/BP_TargettingActor.BP_TargettingActor_C" (`KismetMathLibrary.MakeTransform` (-5000.0 -5000.0 -5000.0)) "Undefined" "MultiplyWithRoot" null null))
      (set `self.TargetingActor` _returnvalue)
      (set `self.bShowMouseCursor` false))))

(fn `UpdateMana`
  (params (ManaUsed :type Integer))
  (bind (_playerstats_visibilityrange _playerstats_mana) (break `/Game/_Main/Actors/Struct/S_PlayerStats` (`self.PlayerStats`)))
  (bind (_playerstats_visibilityrange_2 _playerstats_mana_2 _playerstats_manaperturn _playerstats_tempovermana _playerstats_drawcardperturn _playerstats_maxhandsize) (break `/Game/_Main/Actors/Struct/S_PlayerStats` (`self.PlayerStats`)))
  (set `self.PlayerStats` (make `/Game/_Main/Actors/Struct/S_PlayerStats` _playerstats_visibilityrange_2 (- _playerstats_mana_2 (`local.ManaUsed`)) _playerstats_manaperturn _playerstats_tempovermana _playerstats_drawcardperturn _playerstats_maxhandsize))
  (`/Game/_Main/TCG/Cards/Widget/WBP_Mana.UpdateMana` (`/Game/_Main/TCG/Cards/Widget/WBP_HUD.WBP_Mana` (`self.HUD`)) _playerstats_mana))

(fn `UpdateManaPerTurn`
  (params (ManaPerTurnChange :type Integer))
  (bind (_playerstats_visibilityrange _playerstats_mana _playerstats_manaperturn) (break `/Game/_Main/Actors/Struct/S_PlayerStats` (`self.PlayerStats`)))
  (bind (_playerstats_visibilityrange_2 _playerstats_mana_2 _playerstats_manaperturn_2 _playerstats_tempovermana _playerstats_drawcardperturn _playerstats_maxhandsize) (break `/Game/_Main/Actors/Struct/S_PlayerStats` (`self.PlayerStats`)))
  (set `self.PlayerStats` (make `/Game/_Main/Actors/Struct/S_PlayerStats` _playerstats_visibilityrange_2 _playerstats_mana_2 (+ _playerstats_manaperturn_2 (`local.ManaPerTurnChange`)) _playerstats_tempovermana _playerstats_drawcardperturn _playerstats_maxhandsize))
  (`/Game/_Main/TCG/Cards/Widget/WBP_Mana.UpdateMaxMana` (`/Game/_Main/TCG/Cards/Widget/WBP_HUD.WBP_Mana` (`self.HUD`)) _playerstats_manaperturn))

(fn `UpdatePlayersStats`
  (bind (_playerstats_visibilityrange _playerstats_mana _playerstats_manaperturn _playerstats_tempovermana _playerstats_drawcardperturn _playerstats_maxhandsize) (break `/Game/_Main/Actors/Struct/S_PlayerStats` (`self.PlayerStats`)))
  (set `self.PlayerStats` (make `/Game/_Main/Actors/Struct/S_PlayerStats` _playerstats_visibilityrange (+ _playerstats_manaperturn _playerstats_tempovermana) _playerstats_manaperturn 0 _playerstats_drawcardperturn _playerstats_maxhandsize))
  (`self.UpdateMana` 0)
  (`self.UpdateManaPerTurn` 0))

(fn `UserConstructionScript`)